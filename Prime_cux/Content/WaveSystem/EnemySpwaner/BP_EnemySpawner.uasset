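; Wave-system spawner actor that spawns queued enemy classes at its own transform.
; AddEnemyToQueue appends a class and spawns immediately if no base enemy overlaps its collision sphere, while a looping timer keeps draining the queue without that check.
; Spawned enemies get an elimination binding, with OnEnemyElmination notifying the wave game mode, and are tracked so ClearAllEnemies can destroy them.
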(event `self.ReceiveBeginPlay`
  (`KismetSystemLibrary.K2_SetTimerDelegate` (delegate `SpawnEnemy`) 3.0 true))

(event `SpawnEnemy`
  (`self.SpwanEnemy`)
  (`KismetSystemLibrary.PrintString` "spawn"))

(event `OnEnemyElmination`
  (`/Game/WaveSystem/BP_WaveGameMode.OnEnemeyEliminated` (`/Game/Blueprints/BP_Function_Libary.Get Wave Game Mode`)))

(event `ClearAllEnemies`
  ;[1 1 1] ClearEnemies
  (for _array_element (`self.SpawnEnemies`)
    (`/Engine/EditorBlueprintResources/StandardMacros.IsValid` _array_element
      (:`Is Valid`
        (`self.K2_DestroyActor` _array_element)))))

(fn `AddEnemy To Queue`
  (params (EnemeyClass :type "/Game/AI/Enemy_AI/BP_Enemy_Base Class Reference (by ref)"))
  (`KismetArrayLibrary.Array_Add` (`self.EnemyQueue`) EnemeyClass)
  (if (not (`KismetArrayLibrary.Array_IsValidIndex` (`PrimitiveComponent.GetOverlappingActors` (`self.SphereCollision`) "/Game/AI/Enemy_AI/BP_Enemy_Base.BP_Enemy_Base_C")))
    (`self.SpwanEnemy`)))

(fn `SpwanEnemy`
  (returns (Success :type Boolean))
  (if (`KismetArrayLibrary.Array_IsValidIndex` (`self.EnemyQueue`))
    (bind _returnvalue (`|SpawnActorFromClass` (`|GetArrayItem` (`self.EnemyQueue`)) (`self.GetTransform`) "AdjustIfPossibleButAlwaysSpawn" "MultiplyWithRoot" null 2 null))
    (`/Engine/EditorBlueprintResources/StandardMacros.IsValid` _returnvalue
      (:`Is Valid`
        (add `/Game/AI/Enemy_AI/BP_Enemy_Base.OnEliminated` _returnvalue (`|CreateDelegate` :!event `OnEnemyElmination`))
        (`KismetArrayLibrary.Array_Remove` (`self.EnemyQueue`))
        (`KismetArrayLibrary.Array_Add` (`self.SpawnEnemies`) _returnvalue)
        (`KismetSystemLibrary.PrintString` "SpawnLocationValid" true true (struct :`R` 0.009483 :`G` 0.53125 :`B` 0.184826 :`A` 1.0) 7.0)
        (return true)))
    (else
      (`KismetSystemLibrary.PrintString` "EnemyCantSpawn" true true (struct :`R` 0.40625 :`B` 0.023156 :`A` 1.0) 5.0)
      (return false))))

(fn `UserConstructionScript`)