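; Game mode that runs an enemy wave loop: a five-second interlude, then a timed wave ending on timeout or when all enemies are eliminated.
; Each wave draws its enemy pool from DT_WaveData, falling back to a formula, and lengthens the countdown.
; Random pool picks queue at random spawners up to a concurrent limit, refilling on kills.
; Dispatchers broadcast wave, kill and timer changes.
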(event `self.ReceiveBeginPlay`
  (`self.Interlude`))

(event `Interlude`
  (bind _returnvalue (`KismetSystemLibrary.K2_SetTimerDelegate` (delegate `BeginNextWave`) 5.0))
  (set `self.InterTImer` _returnvalue)
  (`self.EndWave`))

(event `BeginNextWave`
  (`self.StartWave`))

(event `ResetTime`
  ;[1 1 1] WaveTimer
  (goto _label :!via `Reset`))

(event `StartTimer`
  ;[1 1 1] WaveTimer
  (if (== (`self.Sec`) 0)
    (if (== (`self.Min`) 0)
      (`/Engine/EditorBlueprintResources/StandardMacros.DoOnce` false :!label _label
        (:`Completed`
          (if (not (`self.OnBreak`))
            (`self.Interlude`)
            (else
              (set `self.OnBreak` false)))))
      (else
        (set `self.Sec` 59)
        (set `self.Min` (- (`self.Min`) 1))
        (`self.OnTimerUpdated` (`self.Min`) (`self.Sec`) :!label _label_2)))
    (else
      (set `self.Sec` (- (`self.Sec`) 1))
      (goto _label_2))))

(fn `AddEnemyToQueue`
  (`/Game/WaveSystem/EnemySpwaner/BP_EnemySpawner.AddEnemy To Queue` (`KismetArrayLibrary.Array_Random` (`self.EnemySpawners`)) (`self.GetEnemyFromPool`)))

(fn `AlgorithmicWave`
  (bind _enemypoolsize (`self.GetPoolSize`))
  (bind _wavenumber (`self.WaveNumber`))
  (bind _wavenumber_2 (`self.WaveNumber`))
  (`BlueprintMapLibrary.Map_Add` (`self.EnemyPool`) "/Game/AI/Enemy_AI/BP_Enemy_Base.BP_Enemy_Base_C" (`KismetMathLibrary.Clamp` (+ (* _wavenumber_2 _wavenumber_2) 2) 5))
  (`BlueprintMapLibrary.Map_Add` (`self.EnemyPool`) "/Game/AI/Enemy_AI/BP_Enemy_Type1.BP_Enemy_Type1_C" (`KismetMathLibrary.Clamp` (+ (* _wavenumber _wavenumber) 2) 4))
  (set `self.EnemiesRemaining` _enemypoolsize)
  (set `self.TotalEnemies` _enemypoolsize))

(fn `BuildEnemyPool`
  (bind _enemypoolsize (`self.GetPoolSize`))
  (bind _returnvalue (`|GetDataTableRow` "/Game/WaveSystem/WaveData/DT_WaveData.DT_WaveData" (`KismetStringLibrary.Conv_StringToName` (`KismetStringLibrary.Conv_IntToString` (`self.WaveNumber`))))
    (:`then`
      (set `self.EnemyPool` (`.EnemyPool_4_0F4C0B744F9685B48D791CA890F3914F` (break `/Game/WaveSystem/WaveData/S_WaveInfo` _returnvalue)))
      (set `self.EnemiesRemaining` _enemypoolsize)
      (set `self.TotalEnemies` _enemypoolsize))
    (:`RowNotFound`
      (`self.AlgorithmicWave`))))

(fn `BuildWave`
  (`self.BuildEnemyPool`)
  (for _ (range (`KismetMathLibrary.Min` (`self.GetPoolSize`) (`self.EnemiesLimit`)))
    (`self.AddEnemyToQueue`)))

(fn `CountDownTimer`
  (returns (Min :type Integer) (Sec :type Integer))
  (`KismetSystemLibrary.K2_SetTimerDelegate` (`|CreateDelegate` :!event `StartTimer`) 1.0 true)
  (return (`self.Min`) (`self.Sec`)))

(fn `CreateWaveHUD`
  (bind _returnvalue (`|CreateWidget` "/Game/UI/WP_HUD.WP_HUD_C" null null))
  (`UserWidget.AddToViewport` _returnvalue 0))

(fn `EndWave`
  (set `self.EnemiesKilled` 0)
  (set `self.Min` 0)
  (set `self.Sec` 0)
  (for _array_element (`self.EnemySpawners`)
    (`/Game/WaveSystem/EnemySpwaner/BP_EnemySpawner.ClearAllEnemies` _array_element))
  (`self.OnWaveEnd`))

(fn `GetEnemyFromPool`
  (returns (EnemyClass :type "/Game/AI/Enemy_AI/BP_Enemy_Base Class Reference"))
  (locals (Local_EnemyClass :type "/Game/AI/Enemy_AI/BP_Enemy_Base Class Reference"))
  (bind _keys (`BlueprintMapLibrary.Map_Keys` (`self.EnemyPool`)))
  (bind _output_get (set `local.Local_EnemyClass` (`KismetArrayLibrary.Array_Random` _keys)))
  (bind _returnvalue (- (`BlueprintMapLibrary.Map_Find` (`self.EnemyPool`) _output_get) 1))
  (if (<= _returnvalue 0)
    (`BlueprintMapLibrary.Map_Remove` (`self.EnemyPool`) (`local.Local_EnemyClass`))
    (else
      (`BlueprintMapLibrary.Map_Add` (`self.EnemyPool`) (`local.Local_EnemyClass`) _returnvalue)))
  (return (`local.Local_EnemyClass`)))

(fn `GetEnemySpwaner`
  (bind _outactors (`GameplayStatics.GetAllActorsOfClass` "/Game/WaveSystem/EnemySpwaner/BP_EnemySpawner.BP_EnemySpawner_C"))
  (set `self.EnemySpawners` _outactors))

(fn `GetPoolSize`
  (returns (EnemyPoolSize :type Integer))
  (locals (Local_EnemyPool :type Integer))
  (bind _values (`BlueprintMapLibrary.Map_Values` (`self.EnemyPool`)))
  (for _array_element _values
    (set `local.Local_EnemyPool` (+ _array_element (`local.Local_EnemyPool`))))
  (return (`local.Local_EnemyPool`)))

(fn `OnEnemeyEliminated`
  (`/Engine/EditorBlueprintResources/StandardMacros.DecrementInt` (`self.EnemiesRemaining`)
    (:`  `
      (bind _result (`/Engine/EditorBlueprintResources/StandardMacros.IncrementInt` (`self.EnemiesKilled`))
        (:`  `
          (`self.OnEnemyKilled` _result (`self.TotalEnemies`) (`self.Gold Collected`))
          (if (< (`self.EnemiesRemaining`) (`self.EnemiesLimit`))
            (if (== (`self.EnemiesRemaining`) 0)
              (`self.Interlude`)
              (set `self.OnBreak` true))
            (else
              (`self.AddEnemyToQueue`))))))))

(fn `StartWave`
  (`/Engine/EditorBlueprintResources/StandardMacros.IncrementInt` (`self.WaveNumber`)
    (:`  `
      (`self.GetEnemySpwaner`)
      (`self.WaveClock`)
      (`self.BuildWave`)
      (`self.OnStartWave` (`self.WaveNumber`) (`self.EnemiesKilled`) (`self.TotalEnemies`) (`self.Gold Collected`))
      (`self.ResetTime`))))

(fn `UserConstructionScript`)

(fn `WaveClock`
  ;[0.399 0.399 0.399] WaveSeconds(Config)
  (bind _output_get (set `self.StoredSeconds` (+ (`self.StoredSeconds`) 20)))
  (if (>= _output_get 60)
    (set `self.StoredSeconds` 0)
    (bind _result (`/Engine/EditorBlueprintResources/StandardMacros.IncrementInt` (`self.StoredMinutes`))
      (:`  `
        (set `self.Min` _result)))
    (else
      (set `self.Sec` (`self.StoredSeconds`))
      (set `self.Min` (`self.StoredMinutes`)))))