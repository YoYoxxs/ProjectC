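; Base AI controller for enemies that runs the possessed BP_Enemy_Base's behavior tree and drives its state through the Blackboard.
; On possess it starts Passive and copies the pawn's attack and defend radii into the Blackboard.
; Perception updates check sight, hearing and damage: while Passive or Investigating, seeing or being damaged by the player triggers Attack, and sounds set an investigation point.
; Setter functions also provide Dead and Stun states.
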(event `self.ReceiveBeginPlay`
  ;[1 1 1] Comment
)

(event `self.ReceivePossess`
  (params (PossessedPawn :type "Pawn Object Reference"))
  ;[1 1 1] Comment
  (bind _asbp_enemy_base (cast `/Game/Blueprints/AI/BP_Enemy_Base` PossessedPawn))
  (bind _behaviortree (`/Game/Blueprints/AI/BP_Enemy_Base.BehaviorTree` _asbp_enemy_base)
    (:`then`
      (`self.RunBehaviorTree` _behaviortree)
      (`self.SetStateAsPassive`)
      (bind (_attackraduis _deffendraduis) (message `/Game/Blueprints/AI/BI_AI.GetIdealRange` PossessedPawn))
      (`BlackboardComponent.SetValueAsFloat` (`self.Blackboard`) (`self.AttackRaduisKeyName`) _attackraduis)
      (`BlackboardComponent.SetValueAsFloat` (`self.Blackboard`) (`self.DeffendRaduisKeyName`) _deffendraduis))
    (:`else`)))

(event `self.AIPerception.OnPerceptionUpdated`
  (params (UpdatedActors :type "Array of Actor Object Reference (by ref)"))
  (for _array_element UpdatedActors
    (`|ExecutionSequence`
      (:`then_0`
        (bind _sensed (`self.CanSenseActor` _array_element "NewEnumerator1"))
        (if _sensed
          (`self.HandleSensedSight` _array_element)))
      (:`then_1`
        (bind (_sensed_2 _stimulus) (`self.CanSenseActor` _array_element "NewEnumerator2"))
        (if _sensed_2
          (`self.HandleSensedSound` (`.StimulusLocation` (break `AIStimulus` _stimulus)))))
      (:`then_2`
        (bind _sensed_3 (`self.CanSenseActor` _array_element "NewEnumerator3"))
        (if _sensed_3
          (`self.HandleSenseDamage` _array_element))))))

(fn `CanSenseActor`
  (params (Actor :type "Actor Object Reference") (Sense :type "/Game/Blueprints/Enum/E_AI_Sense Enum" :default "NewEnumerator0"))
  (returns (Sensed :type Boolean) (Stimulus :type "AIStimulus Structure"))
  (bind _info (`AIPerceptionComponent.GetActorsPerception` (`self.AIPerception`) Actor))
  (for _array_element (`.LastSensedStimuli` (break `ActorPerceptionBlueprintInfo` _info))
    (bind _returnvalue (`AIPerceptionSystem.GetSenseClassForStimulus` _array_element))
    (if (== _returnvalue (select `/Game/Blueprints/Enum/E_AI_Sense` Sense :`NewEnumerator1` "/Script/AIModule.AISense_Sight" :`NewEnumerator2` "/Script/AIModule.AISense_Hearing" :`NewEnumerator3` "/Script/AIModule.AISense_Damage" :!type "Object Class Reference"))
      (return (`.bSuccessfullySensed` (break `AIStimulus` _array_element)) _array_element))))

(fn `GetCurrentState`
  (returns (State :type "/Game/Blueprints/AI/Enums/E_AIState Enum"))
  (return (cast `/Game/Blueprints/AI/Enums/E_AIState` (`BlackboardComponent.GetValueAsEnum` (`self.Blackboard`) (`self.StateKey Name`)))))

(fn `HandleSenseDamage`
  (params (Actor :type "Actor Object Reference"))
  (bind _state (`self.GetCurrentState`))
  (switch `/Game/Blueprints/AI/Enums/E_AIState` _state
    (:`NewEnumerator1`
      _)
    (:`NewEnumerator2`
      _))
  (if (== Actor (`GameplayStatics.GetPlayerCharacter` 0))
    (`self.SetStateAsAttacking` Actor)))

(fn `HandleSensedSight`
  (params (Actor :type "Actor Object Reference"))
  (bind _state (`self.GetCurrentState`))
  (switch `/Game/Blueprints/AI/Enums/E_AIState` _state
    (:`NewEnumerator1`
      _)
    (:`NewEnumerator2`
      _))
  (if (== Actor (`GameplayStatics.GetPlayerCharacter` 0))
    (`self.SetStateAsAttacking` Actor)))

(fn `HandleSensedSound`
  (params (Location :type "Vector Structure"))
  (bind _state (`self.GetCurrentState`))
  (switch `/Game/Blueprints/AI/Enums/E_AIState` _state
    (:`NewEnumerator1`
      _)
    (:`NewEnumerator2`
      _))
  (`self.SetStateAsInvesigating` Location))

(fn `SetStateAsAttacking`
  (params (AttackingTarget :type "Actor Object Reference") (UseLastKnownAttack :type Boolean))
  (locals (NewAttackTarget :type "Actor Object Reference"))
  (bind _output_get (set `local.NewAttackTarget` (select `bool` (and UseLastKnownAttack (`KismetSystemLibrary.IsValid` (`self.Attacking Target`))) :`false` AttackingTarget :`true` (`self.Attacking Target`))))
  (`/Engine/EditorBlueprintResources/StandardMacros.IsValid` _output_get
    (:`Is Valid`
      (`BlackboardComponent.SetValueAsObject` (`self.Blackboard`) (`self.Attack TargetKey Name`) _output_get)
      (`BlackboardComponent.SetValueAsEnum` (`self.Blackboard`) (`self.StateKey Name`) (enumliteral `/Game/Blueprints/AI/Enums/E_AIState` "NewEnumerator0"))
      (set `self.Attacking Target` (`local.NewAttackTarget`)))))

(fn `SetStateAsDead`
  (`BlackboardComponent.SetValueAsEnum` (`self.Blackboard`) (`self.StateKey Name`) (enumliteral `/Game/Blueprints/AI/Enums/E_AIState` "NewEnumerator6")))

(fn `SetStateAsInvesigating`
  (params (Location :type "Vector Structure"))
  (`BlackboardComponent.SetValueAsEnum` (`self.Blackboard`) (`self.StateKey Name`) (enumliteral `/Game/Blueprints/AI/Enums/E_AIState` "NewEnumerator2"))
  (`BlackboardComponent.SetValueAsVector` (`self.Blackboard`) (`self.PointOfIntrestKeyName`) Location))

(fn `SetStateAsPassive`
  (`BlackboardComponent.SetValueAsEnum` (`self.Blackboard`) (`self.StateKey Name`) (enumliteral `/Game/Blueprints/AI/Enums/E_AIState` "NewEnumerator1")))

(fn `SetStateAsStun`
  (`BlackboardComponent.SetValueAsEnum` (`self.Blackboard`) (`self.StateKey Name`) (enumliteral `/Game/Blueprints/AI/Enums/E_AIState` "NewEnumerator3")))

(fn `UserConstructionScript`)