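; BP_Enemy_Base is the base AI enemy character, with a widget health bar and interface-style functions for team, patrol route, combat ranges and movement speed.
; Health, damage and healing are delegated to BPCDamageSystem.
; Hit responses stun the enemy through AIC_Enemy_Base, then target the attacker after the montage; death plays sound and montage, stops AI logic and destroys it.
; Player line-of-sight, knockback and item-drop logic are disconnected or empty.
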(event `self.ReceiveBeginPlay`
  ;[0 0.1851 1] Comment
  (bind _asaic_enemy_base (cast `/Game/Blueprints/AI/AIC_Enemy_Base` (`AIBlueprintHelperLibrary.GetAIController` self)))
  (set `self.As AIC Enemy Base` _asaic_enemy_base)
  (bind _returnvalue (`|CreateWidget` "/Game/UI/Widgets/WG_HealthBar.WG_HealthBar_C" null self))
  (bind _output_get (set `self.EnemyHealthBar` _returnvalue))
  (`WidgetComponent.SetWidget` (`self.Widget`) _output_get)
  (add `/Game/DamageSys/BPC_DamageSystem.OnDeath` (`self.BPC_DamageSystem`) (`|CreateDelegate` :!event `Death`))
  (add `/Game/DamageSys/BPC_DamageSystem.OnDamageResponse` (`self.BPC_DamageSystem`) (`|CreateDelegate` :!event `HitResponse`)))

(event `LookForPlayer`
  ;[0 0.1851 1] Comment
  (bind _outhit (`KismetSystemLibrary.LineTraceSingle` (`self.K2_GetActorLocation`) (`self.K2_GetActorLocation` (`GameplayStatics.GetPlayerPawn` 0)) "TraceTypeQuery1"))
  (if (== (`.HitActor` (`GameplayStatics.BreakHitResult` _outhit)) (`GameplayStatics.GetPlayerPawn` 0))
    _))

(event `HitResponse`
  (params (DamageResponse :type "/Game/DamageSys/E_DamageResponses Enum" :default "NewEnumerator0") (DamageCasur :type "Actor Object Reference"))
  ;[1 1 1] GetDamaged
  (`MovementComponent.StopMovementImmediately` (`self.CharacterMovement`))
  (`/Game/Blueprints/AI/AIC_Enemy_Base.SetStateAsStun` (`self.As AIC Enemy Base`))
  (`|PlayMontage` (`self.Mesh`) (`self.HitReactionMontage`)
    (:`OnCompleted`
      _)
    (:`OnInterrupted`
      _))
  (`/Game/Blueprints/AI/AIC_Enemy_Base.SetStateAsAttacking` (`self.As AIC Enemy Base`) DamageCasur true))

(event `Death`
  ;[1 1 1] GetDamaged
  (`GameplayStatics.PlaySound2D` "/Game/Assest/DungeonResourcePack/Content/Sounds/Hit-death/261419__archeos__womanscream.261419__archeos__womanscream" 1.0 1.0 0.0 null null)
  (`|PlayMontage` (`self.Mesh`) "/Game/Blueprints/AI/Death_Forward2_Montage.Death_Forward2_Montage"
    (:`OnCompleted`
      _)
    (:`OnInterrupted`
      _))
  (`BrainComponent.StopLogic` (`AIController.BrainComponent` (`self.As AIC Enemy Base`)) "")
  (`/Game/Blueprints/AI/AIC_Enemy_Base.SetStateAsDead` (`self.As AIC Enemy Base`))
  (`self.K2_DestroyActor`))

(event `self.Sphere.OnComponentBeginOverlap`
  (params (OverlappedComponent :type "PrimitiveComponent Object Reference") (OtherActor :type "Actor Object Reference") (OtherComp :type "PrimitiveComponent Object Reference") (OtherBodyIndex :type Integer) (bFromSweep :type Boolean) (SweepResult :type "HitResult Structure (by ref)"))
  (if (`ActorComponent.ComponentHasTag` OtherComp "P")
    (`KismetSystemLibrary.K2_UnPauseTimerHandle` (struct))))

(event `self.Sphere.OnComponentEndOverlap`
  (params (OverlappedComponent :type "PrimitiveComponent Object Reference") (OtherActor :type "Actor Object Reference") (OtherComp :type "PrimitiveComponent Object Reference") (OtherBodyIndex :type Integer))
  (if (`ActorComponent.ComponentHasTag` OtherComp "P")
    _))

(event `/Game/Blueprints/AI/BI_AI.KnockBack`
  (params (Direction :type "Vector Structure")))

(fn `CurrentHealth`
  (returns (CurrentHealth :type "Float (double-precision)"))
  (return (`/Game/DamageSys/BPC_DamageSystem.Health` (`self.BPC_DamageSystem`))))

(fn `Get PetrolRaoute`
  (returns (PetrolRoute :type "/Game/Blueprints/AI/BP_PetrolRaote Object Reference"))
  (return (`self.PatrolRoute`)))

(fn `GetIdealRange`
  (returns (AttackRaduis :type "Float (double-precision)") (DeffendRaduis :type "Float (double-precision)"))
  (return 150.0 350.0))

(fn `GetTeamNumber`
  (returns (TeamNumber :type Integer))
  (return 0))

(fn `Heal`
  (params (Amount :type "Float (double-precision)"))
  (returns (NewHealth :type "Float (double-precision)"))
  (bind _newhealth (`/Game/DamageSys/BPC_DamageSystem.Heal` (`self.BPC_DamageSystem`) Amount))
  (return _newhealth))

(fn `IsDead`
  (returns (Dead :type Boolean))
  (return (`/Game/DamageSys/BPC_DamageSystem.IsDead` (`self.BPC_DamageSystem`))))

(fn `MaxHealth`
  (returns (MaxHealth :type "Float (double-precision)"))
  (return (`/Game/DamageSys/BPC_DamageSystem.MaxHealth` (`self.BPC_DamageSystem`))))

(fn `SetMovementSpeed`
  (params (Speed :type "/Game/Blueprints/AI/Enums/E_AI_MovementSpeed Enum" :default "NewEnumerator0"))
  (returns (SpeedValue :type "Float (double-precision)"))
  (bind _output_get (set `CharacterMovementComponent.MaxWalkSpeed` (select `/Game/Blueprints/AI/Enums/E_AI_MovementSpeed` Speed :`NewEnumerator1` 100.0 :`NewEnumerator2` 300.0 :`NewEnumerator3` 500.0 :!type "Float (single-precision)") (`self.CharacterMovement`)))
  (return _output_get))

(fn `TakeDamage`
  (params (DamageInfo :type "/Game/DamageSys/S_DamageInfo Structure") (`Damage Casuer` :type "Actor Object Reference"))
  (returns (WasDamaged :type Boolean))
  (bind _wasdamaged (`/Game/DamageSys/BPC_DamageSystem.TakeDamage` (`self.BPC_DamageSystem`) DamageInfo `Damage Casuer`))
  (return _wasdamaged))

(fn `UserConstructionScript`)