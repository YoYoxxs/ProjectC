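; BP_Enemy_Mele is a melee enemy that equips, unequips and attacks with a sword.
; Montage notifies time the sword's spawn and attachment to the hand socket, its removal, and the attack hit check.
; The attack sphere-traces forward for pawns and sends damage through a TakeDamage message, with debug drawing and printing left on.
; Montage completion fires equip, unequip and attack-end dispatchers, with attack end also firing on interruption.
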(event `self.ReceiveBeginPlay`
  (`parent.ReceiveBeginPlay`))

(event `/Game/Blueprints/AI/BI_AI.EquipWeapon`
  (bind _notifyname (`|PlayMontage` (`self.Mesh`) "/Game/Animation/pose_animations/WieldSwordAnimation_Montage.WieldSwordAnimation_Montage")
    (:`OnCompleted`
      (`self.OnWeaponEquipped`))
    (:`OnNotifyBegin`
      (switch `name` _notifyname
        (:`HoldSword`
          (bind _returnvalue (`|SpawnActorFromClass` "/Game/Blueprints/Wepons/BP_Sword.BP_Sword_C" (`self.GetTransform`) "Undefined" "MultiplyWithRoot" null null))
          (bind _output_get (set `self.WeaponActor` _returnvalue))
          (`self.K2_AttachToComponent` _output_get (`self.Mesh`) "hand_Sword_rSocket" "SnapToTarget" "SnapToTarget" "SnapToTarget" true)
          (set `self.IsWieldingWeapon` true))))))

(event `/Game/Blueprints/AI/BI_AI.UnequipWeapon`
  (bind _notifyname (`|PlayMontage` (`self.Mesh`) "/Game/Animation/pose_animations/WieldSwordAnimation_Montage.WieldSwordAnimation_Montage")
    (:`OnCompleted`
      (`self.OnWeaponUnequipped`))
    (:`OnNotifyBegin`
      (switch `name` _notifyname
        (:`HoldSword`
          (`self.K2_DestroyActor` (`self.WeaponActor`))
          (set `self.IsWieldingWeapon` false))))))

(event `/Game/Blueprints/AI/BI_AI.Attacking`
  (bind _returnvalue (`self.K2_GetActorLocation`))
  (`KismetSystemLibrary.PrintString` "EnemyAttack")
  (bind _notifyname (`|PlayMontage` (`self.Mesh`) "/Game/Animation/PrimaryAttack_D_Slow_Montage.PrimaryAttack_D_Slow_Montage")
    (:`OnCompleted`
      (`self.OnAttackEnd` :!label _label))
    (:`OnInterrupted`
      (goto _label))
    (:`OnNotifyBegin`
      (switch `name` _notifyname
        (:`Sweep`
          (bind (_outhit _returnvalue_2) (`KismetSystemLibrary.SphereTraceSingleForObjects` :`Start` _returnvalue :`End` (+ (* (`self.GetActorForwardVector`) 200.0) _returnvalue) :`Radius` 20.0 :`ObjectTypes` (`|MakeArray` "ObjectTypeQuery3" :!type "EObjectTypeQuery Enum") :`DrawDebugType` "ForDuration"))
          (if _returnvalue_2
            (message `/Game/DamageSys/BPI_Damagable.TakeDamage` (`.HitActor` (`GameplayStatics.BreakHitResult` _outhit)) (make `/Game/DamageSys/S_DamageInfo` 12.5 "NewEnumerator1"))))))))

(fn `UserConstructionScript`
  (`parent.UserConstructionScript`))