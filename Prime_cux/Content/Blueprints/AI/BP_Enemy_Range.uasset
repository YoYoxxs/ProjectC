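; Ranged enemy character that throws daggers at its target, with an ideal attack and defend range for AI.
; Montage notifies time weapon spawning, destruction and throws, while montage endings fire equip, unequip and attack-end events.
; A throw requires a clear visibility trace to the AI controller's attack target, but the dagger's velocity aims at player 0.
; Health, healing and damage functions forward to BPCDamageSystem, and SetMovementSpeed maps states to walk speeds.
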(event `self.ReceiveBeginPlay`
  (`parent.ReceiveBeginPlay`))

(event `/Game/Blueprints/AI/BI_AI.UnequipWeapon`
  ;[1 1 1] Combat
  (bind _notifyname (`|PlayMontage` (`self.Mesh`) "/Game/Animation/Emote_SwordSwallow_Montage.Emote_SwordSwallow_Montage")
    (:`OnCompleted`
      (`self.OnWeaponUnequipped` :!label _label))
    (:`OnInterrupted`
      (goto _label))
    (:`OnNotifyBegin`
      (switch `name` _notifyname
        (:`HoldSword`
          (`self.K2_DestroyActor` (`self.WeaponActor`))
          (set `self.IsWieldingWeapon` false))))))

(event `/Game/Blueprints/AI/BI_AI.EquipWeapon`
  ;[1 1 1] Combat
  (bind _notifyname (`|PlayMontage` (`self.Mesh`) "/Game/Animation/Emote_SwordSwallow_Montage.Emote_SwordSwallow_Montage")
    (:`OnCompleted`
      (`self.OnWeaponEquipped` :!label _label_2))
    (:`OnInterrupted`
      (goto _label_2))
    (:`OnNotifyBegin`
      (switch `name` _notifyname
        (:`HoldSword`
          (bind _returnvalue (`|SpawnActorFromClass` "/Game/Blueprints/Ability/Projectile/BP_Dagger.BP_Dagger_C" (`self.GetTransform`) "Undefined" "MultiplyWithRoot" null (0.0 0.0 0.0) null))
          (set `self.Dagger` _returnvalue)
          (`self.K2_AttachToComponent` (`self.Mesh`) "hand_Dagger_rSocket" "SnapToTarget" "SnapToTarget" "SnapToTarget")
          (set `self.IsWieldingWeapon` true))))))

(event `/Game/Blueprints/AI/BI_AI.Shoot`
  ;[1 1 1] Combat
)

(event `/Game/Blueprints/AI/BI_AI.Attacking`
  (bind _returnvalue (`SceneComponent.GetSocketLocation` (`self.Mesh`) "weapon_r"))
  ;[1 1 1] Combat
  (bind _notifyname (`|PlayMontage` (`self.Mesh`) "/Game/Animation/Combat_Animations/PrimaryAttack_A_Slow_Montage.PrimaryAttack_A_Slow_Montage")
    (:`OnCompleted`
      (`self.OnAttackEnd` :!label _label_3))
    (:`OnInterrupted`
      (goto _label_3))
    (:`OnNotifyBegin`
      (switch `name` _notifyname
        (:`Dagger`
          (bind _asaic_enemy_base (cast `/Game/Blueprints/AI/AIC_Enemy_Base` (`AIBlueprintHelperLibrary.GetAIController` self)))
          (bind _attacking_target (`/Game/Blueprints/AI/AIC_Enemy_Base.Attacking Target` _asaic_enemy_base)
            (:`then`
              (bind (_outhit _returnvalue_2) (`KismetSystemLibrary.LineTraceSingle` :`Start` (`self.K2_GetActorLocation`) :`End` (`self.K2_GetActorLocation` _attacking_target) :`TraceChannel` "TraceTypeQuery1" :`DrawDebugType` "ForDuration"))
              (if (not _returnvalue_2)
                (`|SpawnActorFromClass` "/Game/Blueprints/Ability/Projectile/BP_Dagger.BP_Dagger_C" (`KismetMathLibrary.MakeTransform` _returnvalue) "Undefined" "MultiplyWithRoot" null (* (`KismetMathLibrary.GetForwardVector` (`KismetMathLibrary.FindLookAtRotation` _returnvalue (`self.K2_GetActorLocation` (`GameplayStatics.GetPlayerPawn` 0)))) 1200) null)
                (`KismetSystemLibrary.PrintString` "Dagger Damage")))
            (:`else`)))))))

(fn `CurrentHealth`
  (returns (CurrentHealth :type "Float (double-precision)"))
  (return (`/Game/DamageSys/BPC_DamageSystem.Health` (`self.BPC_DamageSystem`))))

(fn `GetIdealRange`
  (returns (AttackRaduis :type "Float (double-precision)") (DeffendRaduis :type "Float (double-precision)"))
  (return 600.0 600.0))

(fn `Heal`
  (params (Amount :type "Float (double-precision)"))
  (returns (NewHealth :type "Float (double-precision)"))
  (bind _newhealth (`/Game/DamageSys/BPC_DamageSystem.Heal` (`self.BPC_DamageSystem`) Amount))
  (return _newhealth))

(fn `IsDead`
  (returns (Dead :type Boolean))
  (return (`/Game/DamageSys/BPC_DamageSystem.IsDead` (`self.BPC_DamageSystem`))))

(fn `MaxHealth`
  (returns (MaxHealth :type "Float (double-precision)"))
  (return (`/Game/DamageSys/BPC_DamageSystem.MaxHealth` (`self.BPC_DamageSystem`))))

(fn `SetMovementSpeed`
  (params (Speed :type "/Game/Blueprints/AI/Enums/E_AI_MovementSpeed Enum" :default "NewEnumerator0"))
  (returns (SpeedValue :type "Float (double-precision)"))
  (set `CharacterMovementComponent.MaxWalkSpeed` (select `/Game/Blueprints/AI/Enums/E_AI_MovementSpeed` Speed :`NewEnumerator1` 200.0 :`NewEnumerator2` 300.0 :`NewEnumerator3` 500.0 :!type "Float (single-precision)") (`self.CharacterMovement`))
  (return 0.0))

(fn `TakeDamage`
  (params (DamageInfo :type "/Game/DamageSys/S_DamageInfo Structure") (`Damage Casuer` :type "Actor Object Reference"))
  (returns (WasDamaged :type Boolean))
  (bind _wasdamaged (`/Game/DamageSys/BPC_DamageSystem.TakeDamage` (`self.BPC_DamageSystem`) DamageInfo null))
  (return _wasdamaged))

(fn `UserConstructionScript`
  (`parent.UserConstructionScript`))