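; Boss orb actor that carries its own health through a damage system component, initialized to full in the construction script.
; TakeDamage forwards hits to that component and returns its result.
; A Respawn event spawns a BP_Boss_Orbs actor at a random point within its Box bounds with a preset current health.
; BeginPlay calls TakeDamage without inputs, and its zero-health check leads to no action.
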(event `self.ReceiveBeginPlay`
  (`parent.ReceiveBeginPlay`)
  (bind _wasdamaged (`self.TakeDamage` (struct)))
  (if _wasdamaged
    (if (<= (`/Game/DamageSys/BPC_DamageSystem.Health` (`self.BPC_DamageSystem`)) 0.0)
      _)))

(event `Respawn`
  (bind _box (`self.Box`))
  (`|SpawnActorFromClass` "/Game/Blueprints/AI/Boss/BP_Boss_Orbs.BP_Boss_Orbs_C" (`KismetMathLibrary.MakeTransform` (`KismetMathLibrary.RandomPointInBoundingBox` (`SceneComponent.K2_GetComponentLocation` _box) (`BoxComponent.BoxExtent` _box))) "Undefined" "MultiplyWithRoot" null null null 31.0))

(fn `TakeDamage`
  (params (DamageInfo :type "/Game/DamageSys/S_DamageInfo Structure") (`Damage Casuer` :type "Actor Object Reference"))
  (returns (WasDamaged :type Boolean))
  (bind _wasdamaged (`/Game/DamageSys/BPC_DamageSystem.TakeDamage` (`self.BPC_DamageSystem`) DamageInfo `Damage Casuer`))
  (return _wasdamaged))

(fn `UserConstructionScript`
  (bind _bpc_damagesystem (`self.BPC_DamageSystem`))
  (`parent.UserConstructionScript`)
  (bind _output_get (set `/Game/DamageSys/BPC_DamageSystem.MaxHealth` 80.0 _bpc_damagesystem))
  (set `/Game/DamageSys/BPC_DamageSystem.Health` _output_get _bpc_damagesystem))