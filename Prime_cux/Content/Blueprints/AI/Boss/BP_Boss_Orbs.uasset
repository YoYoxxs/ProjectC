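; Boss orb actor that relays damage to BP_Boss and replaces itself when destroyed.
; Each hit lowers its clamped health; non-lethal hits apply the same damage to the BP_Boss found by class lookup and print debug messages.
; At zero health it spawns a new orb at a random point inside its Box bounds, then destroys itself after a short delay.
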(event `self.ReceiveBeginPlay`
  (set `self.CurrentHealth` (`self.MaxHealth`)))

(event `self.ReceiveAnyDamage`
  (params (Damage :type "Float (single-precision)") (DamageType :type "DamageType Object Reference") (InstigatedBy :type "Controller Object Reference") (DamageCauser :type "Actor Object Reference"))
  (bind _output_get (set `self.CurrentHealth` (`KismetMathLibrary.FClamp` (- (`self.CurrentHealth`) Damage) 0.0 (`self.MaxHealth`))))
  (if (<= _output_get 0.0)
    (`self.ReSpawn`)
    (`KismetSystemLibrary.Delay` 0.2)
    (`self.K2_DestroyActor`)
    (else
      (`KismetSystemLibrary.PrintString` "Got hit")
      (bind _returnvalue (`GameplayStatics.GetActorOfClass` "/Game/Blueprints/AI/Boss/BP_Boss.BP_Boss_C"))
      (`GameplayStatics.ApplyDamage` _returnvalue Damage)
      (`KismetSystemLibrary.PrintString` "Boss Got Damaged"))))

(event `ReSpawn`
  (bind _box (`self.Box`))
  (`|SpawnActorFromClass` "BP_Boss_Orbs_C" (`KismetMathLibrary.MakeTransform` (`KismetMathLibrary.RandomPointInBoundingBox` (`SceneComponent.K2_GetComponentLocation` _box) (`BoxComponent.BoxExtent` _box))) "Undefined" "MultiplyWithRoot" null 31.0 31.0 null null))

(fn `UserConstructionScript`
  (`parent.UserConstructionScript`))