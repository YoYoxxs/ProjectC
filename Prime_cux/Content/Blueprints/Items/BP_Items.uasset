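; World item pickup that takes its mesh and name from a DT_Items row and goes into the inventory on interaction.
; On spawn, repeated random sphere traces pick a nearby landing point, preferring "F"-tagged surfaces, then a timeline scales and arcs the item there.
; A name widget follows hover and the player's item-visibility toggle.
; Interacting within the overlap sphere calls the game mode's AddToInventory, destroying the item on success or bouncing it on failure.
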(event `ShowWidget`
  (`/Game/UI/Widgets/WG_ItemWorld.SetText` (cast `/Game/UI/Widgets/WG_ItemWorld` (`WidgetComponent.GetWidget` (`self.Widget`)) :!pure true) (`KismetTextLibrary.Conv_StringToText` (`.ItemName_2_F8550BE6469FDDF4726319BC8FE17F7A` (break `/Game/Blueprints/Items/ST_Items` (`self.ItemData`)))))
  (add `/Game/Blueprints/BP_Player.ToggleItems` (cast `/Game/Blueprints/BP_Player` (`GameplayStatics.GetPlayerCharacter` 0) :!pure true) (delegate `ShowItemBind`)))

(event `ShowItemBind`
  (params (ItemVisibility :type Boolean) (AltPresseed :type Boolean))
  (`self.WidgetVisibility` ItemVisibility)
  (set `self.Alt Presseed` AltPresseed))

(event `ItemAnimation`
  (bind _originalitemlocation (`self.OriginalItemLocation`))
  (`SceneComponent.SetHiddenInGame` (`self.ItemMesh`) false false)
  (set `self.OriginalItemLocation` (`self.K2_GetActorLocation`))
  (bind (_direction _movementalpha _newtrack_1) (`Timeline|Timeline` :!via `PlayFromStart`)
    (:`Update`
      (`SceneComponent.SetWorldScale3D` (`self.ItemMesh`) (`KismetMathLibrary.VLerp` (0.0 0.0 0.0) (1.0 1.0 1.0) _newtrack_1))
      (`self.K2_SetActorLocation` (`KismetMathLibrary.VLerp` (select `bool` (< _movementalpha 0.5) :`false` (`self.TargetLocation`) :`true` _originalitemlocation) (+ _originalitemlocation (0.0 0.0 200.0)) _movementalpha) false true))
    (:`Finished`
      (`self.K2_SetActorLocation` (`self.TargetLocation`) false true))))

(event `self.ReceiveBeginPlay`
  (bind _returnvalue (`self.K2_GetActorLocation`))
  (while (== (`self.TargetLocation`) (0.0 0.0 0.0))
    (set `self.Trys` (+ (`self.Trys`) 1))
    (bind _outhit (`KismetSystemLibrary.SphereTraceSingle` (+ _returnvalue (0.0 0.0 200.0)) (+ (* (`self.GetActorUpVector`) -500) (`KismetMathLibrary.RandomPointInBoundingBox` _returnvalue (800.0 800.0 1.0))) 0.0 "TraceTypeQuery2"))
    (bind (_bblockinghit _binitialoverlap _time _distance _location _impactpoint _normal _impactnormal _physmat _hitactor _hitcomponent) (`GameplayStatics.BreakHitResult` _outhit))
    (if (or (`ActorComponent.ComponentHasTag` _hitcomponent "F") (== (`self.Trys`) 30))
      (set `self.TargetLocation` _impactpoint)))
  (`|ExecutionSequence`
    (:`then_0`
      (`self.ItemAnimation`))
    (:`then_1`
      (`self.ShowWidget`))))

(event `self.Sphere.OnComponentBeginOverlap`
  (params (OverlappedComponent :type "PrimitiveComponent Object Reference") (OtherActor :type "Actor Object Reference") (OtherComp :type "PrimitiveComponent Object Reference") (OtherBodyIndex :type Integer) (bFromSweep :type Boolean) (SweepResult :type "HitResult Structure (by ref)"))
  (if (`ActorComponent.ComponentHasTag` OtherComp "P")
    (set `self.AbleToPick` true)))

(event `/Game/Blueprints/BI/BI_ItemComponant.Interact`
  (params (PlayerRef :type "/Game/Blueprints/BP_Player Object Reference"))
  (bind _targetlocation (`self.TargetLocation`))
  (`/Engine/EditorBlueprintResources/StandardMacros.IsValid` PlayerRef
    (:`Is Valid`
      (if (and (`self.AbleToPick`) (not (`self.Interacting`)))
        (set `self.Interacting` true)
        (bind _picked (`/Game/Blueprints/BP_WaveGameMode.AddToInventory` (cast `/Game/Blueprints/BP_WaveGameMode` (`GameplayStatics.GetGameMode`) :!pure true) (`self.Row Name`)))
        (if _picked
          (`self.K2_DestroyActor`)
          (else
            (bind (_direction _newtrack_0) (`Timeline|Timeline_0` :!via `PlayFromStart`)
              (:`Update`
                (`self.K2_SetActorLocation` (`KismetMathLibrary.VLerp` _targetlocation (+ _targetlocation (0.0 0.0 150.0)) _newtrack_0) false true))
              (:`Finished`
                (set `self.Interacting` false)))))))))

(event `self.Sphere.OnComponentEndOverlap`
  (params (OverlappedComponent :type "PrimitiveComponent Object Reference") (OtherActor :type "Actor Object Reference") (OtherComp :type "PrimitiveComponent Object Reference") (OtherBodyIndex :type Integer))
  (if (`ActorComponent.ComponentHasTag` OtherComp "P")
    (set `self.AbleToPick` false)))

(event `/Game/Blueprints/BI/BI_ItemComponant.StartHover`
  (params (IsHovered :type Boolean) (PlayerRef :type "/Game/Blueprints/BP_Player Object Reference"))
  (`/Engine/EditorBlueprintResources/StandardMacros.IsValid` PlayerRef
    (:`Is Valid`
      (`self.WidgetVisibility` IsHovered))))

(event `/Game/Blueprints/BI/BI_ItemComponant.EndHover`
  (if (not (`PlayerController.IsInputKeyDown` (`GameplayStatics.GetPlayerController` 0) "LeftAlt"))
    (`self.WidgetVisibility` false)))

(fn `UserConstructionScript`
  (bind _returnvalue (`|GetDataTableRow` "/Game/Blueprints/Items/DT_Items.DT_Items" (`self.Row Name`))
    (:`then`
      (bind _output_get (set `self.ItemData` _returnvalue))
      (`StaticMeshComponent.SetStaticMesh` (`self.ItemMesh`) (`.Mesh_5_460551F8485A00DB969DBE917038B0FF` (break `/Game/Blueprints/Items/ST_Items` _output_get))))))

(fn `WidgetVisibility`
  (params (bNewVisibility :type Boolean))
  (bind _widget (`self.Widget`))
  (`SceneComponent.SetVisibility` _widget bNewVisibility false)
  (bind _output_get (set `PrimitiveComponent.bGenerateOverlapEvents` bNewVisibility _widget))
  (`PrimitiveComponent.SetCollisionEnabled` _widget (select `bool` _output_get :`false` "NoCollision" :`true` "QueryOnly" :!type "ECollisionEnabled Enum"))
  (`WidgetBlueprintLibrary.SetInputMode_GameAndUIEx` (`GameplayStatics.GetPlayerController` 0) (`WidgetComponent.GetWidget` _widget) "DoNotLock" false))