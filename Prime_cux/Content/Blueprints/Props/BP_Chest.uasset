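; BP_Chest is a lootable chest prop for the generated maze, labeled by a world widget and opened once through Interact.
; A sphere overlap with a "P"-tagged component enables opening, which plays a sound, removes the label and swings the lid via Timeline.
; It then spawns one default BP_Items plus a random number of random-row items, capped by MazeGen's level, and registers each in MazeGen's ActorToDestroy list.
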(event `self.ReceiveBeginPlay`
  (set `self.MaxNumberOfItems` (`KismetMathLibrary.RandomIntegerInRange` 1 (+ (`/Game/Blueprints/BP_MazeGen.GeneratorLevel` (`self.MazeGen`)) 1)))
  (`/Game/UI/Widgets/WG_ItemWorld.SetText` (cast `/Game/UI/Widgets/WG_ItemWorld` (`WidgetComponent.GetWidget` (`self.Widget`)) :!pure true) "Chest"))

(event `self.Sphere.OnComponentBeginOverlap`
  (params (OverlappedComponent :type "PrimitiveComponent Object Reference") (OtherActor :type "Actor Object Reference") (OtherComp :type "PrimitiveComponent Object Reference") (OtherBodyIndex :type Integer) (bFromSweep :type Boolean) (SweepResult :type "HitResult Structure (by ref)"))
  (if (`ActorComponent.ComponentHasTag` OtherComp "P")
    (set `self.AbleToPick` true)))

(event `self.Sphere.OnComponentEndOverlap`
  (params (OverlappedComponent :type "PrimitiveComponent Object Reference") (OtherActor :type "Actor Object Reference") (OtherComp :type "PrimitiveComponent Object Reference") (OtherBodyIndex :type Integer))
  (if (`ActorComponent.ComponentHasTag` OtherComp "P")
    (set `self.AbleToPick` false)))

(event `/Game/Blueprints/BI/BI_ItemComponant.Interact`
  (params (PlayerRef :type "/Game/Blueprints/BP_Player Object Reference"))
  (bind _returnvalue (`self.K2_GetActorLocation`))
  (bind _widget (`self.Widget`))
  (bind _actortodestroy (`/Game/Blueprints/BP_MazeGen.ActorToDestroy` (`self.MazeGen`)))
  (`KismetSystemLibrary.PrintString` "opeining")
  (if (and (`self.AbleToPick`) (not (`self.Interacting`)))
    (set `self.Interacting` true)
    (`GameplayStatics.PlaySound2D` "/Game/Assest/DungeonResourcePack/Content/Sounds/Chest/391947__ssierra1202__chest-openning-crack_Cue.391947__ssierra1202__chest-openning-crack_Cue" 1.0 1.0 0.0 null null)
    (`SceneComponent.SetHiddenInGame` _widget true false)
    (`ActorComponent.K2_DestroyComponent` _widget)
    (bind (_direction _newtrack_0) (`Timeline|Timeline` :!via `PlayFromStart`)
      (:`Update`
        (`SceneComponent.K2_SetRelativeRotation` (`self.StaticMesh1`) (`KismetMathLibrary.RLerp` (struct :`Roll` 90.0) (struct :`Roll` -20.0) _newtrack_0 true) false false))
      (:`Finished`
        (bind _returnvalue_2 (`|SpawnActorFromClass` "/Game/Blueprints/Items/BP_Items.BP_Items_C" (`KismetMathLibrary.MakeTransform` _returnvalue) "Undefined" "MultiplyWithRoot" null "I6" null))
        (`KismetArrayLibrary.Array_Add` _actortodestroy _returnvalue_2)
        (for _ (range 1 (+ (`self.MaxNumberOfItems`) 1))
          (bind _returnvalue_3 (`|SpawnActorFromClass` "/Game/Blueprints/Items/BP_Items.BP_Items_C" (`KismetMathLibrary.MakeTransform` _returnvalue) "Undefined" "MultiplyWithRoot" null (`KismetStringLibrary.Conv_StringToName` (`KismetStringLibrary.Concat_StrStr` "I" (`KismetStringLibrary.Conv_IntToString` (`KismetMathLibrary.RandomIntegerInRange` 1 5)))) null))
          (`KismetArrayLibrary.Array_Add` _actortodestroy _returnvalue_3))))))

(fn `UserConstructionScript`)

(fn `WidgetVisibility`
  (params (bNewVisibility :type Boolean))
  (bind _widget (`self.Widget`))
  (`/Engine/EditorBlueprintResources/StandardMacros.IsValid` _widget
    (:`Is Valid`
      (`SceneComponent.SetVisibility` _widget bNewVisibility false)
      (bind _output_get (set `PrimitiveComponent.bGenerateOverlapEvents` bNewVisibility _widget))
      (`PrimitiveComponent.SetCollisionEnabled` _widget (select `bool` _output_get :`false` "NoCollision" :`true` "QueryOnly" :!type "ECollisionEnabled Enum")))))