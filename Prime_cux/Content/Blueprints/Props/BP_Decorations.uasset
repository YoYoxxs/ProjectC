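; Child actor of BP_Tile that dresses one dungeon tile with walls, doors, signs and a collapsible ceiling.
; Generation functions open walls from the tile's direction map, randomize meshes per wall style and add signed doorways, matching components by direction tag.
; Player overlaps update current tile coordinates, while door triggers ask the tile's generator to hide or show room ceilings.
; HideC and ShowC_1 animate the ceiling with a reversible scale timeline.
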(event `self.ReceiveBeginPlay`
  (bind _asbp_tile (cast `/Game/Blueprints/Props/BP_Tile` (`self.GetParentActor`)))
  (set `self.As BP Tile` _asbp_tile))

(event `self.Box.OnComponentBeginOverlap`
  (params (OverlappedComponent :type "PrimitiveComponent Object Reference") (OtherActor :type "Actor Object Reference") (OtherComp :type "PrimitiveComponent Object Reference") (OtherBodyIndex :type Integer) (bFromSweep :type Boolean) (SweepResult :type "HitResult Structure (by ref)"))
  (if (`ActorComponent.ComponentHasTag` OtherComp "P")
    (bind _asbp_player (cast `/Game/Blueprints/BP_Player` OtherActor))
    (set `/Game/Blueprints/BP_Player.CurrentCoords` (`/Game/Blueprints/Props/BP_Tile.TileCoords` (`self.As BP Tile`)) _asbp_player)))

(event `self.SouthDoor.OnComponentBeginOverlap`
  (params (OverlappedComponent :type "PrimitiveComponent Object Reference") (OtherActor :type "Actor Object Reference") (OtherComp :type "PrimitiveComponent Object Reference") (OtherBodyIndex :type Integer) (bFromSweep :type Boolean) (SweepResult :type "HitResult Structure (by ref)"))
  (if (`ActorComponent.ComponentHasTag` OtherComp "P")
    (if (`SceneComponent.IsVisible` (`self.Ceiling`)) :!label _label
      (`/Game/Blueprints/BP_MazeGen.HideRoomC` (`/Game/Blueprints/Props/BP_Tile.Genrator` (`self.As BP Tile`)) (`self.Room Index`)))))

(event `self.NorthDoor.OnComponentBeginOverlap`
  (params (OverlappedComponent :type "PrimitiveComponent Object Reference") (OtherActor :type "Actor Object Reference") (OtherComp :type "PrimitiveComponent Object Reference") (OtherBodyIndex :type Integer) (bFromSweep :type Boolean) (SweepResult :type "HitResult Structure (by ref)"))
  (if (`ActorComponent.ComponentHasTag` OtherComp "P")
    (goto _label)))

(event `self.EastDoor.OnComponentBeginOverlap`
  (params (OverlappedComponent :type "PrimitiveComponent Object Reference") (OtherActor :type "Actor Object Reference") (OtherComp :type "PrimitiveComponent Object Reference") (OtherBodyIndex :type Integer) (bFromSweep :type Boolean) (SweepResult :type "HitResult Structure (by ref)"))
  (if (`ActorComponent.ComponentHasTag` OtherComp "P")
    (goto _label)))

(event `self.WestDoor.OnComponentBeginOverlap`
  (params (OverlappedComponent :type "PrimitiveComponent Object Reference") (OtherActor :type "Actor Object Reference") (OtherComp :type "PrimitiveComponent Object Reference") (OtherBodyIndex :type Integer) (bFromSweep :type Boolean) (SweepResult :type "HitResult Structure (by ref)"))
  (if (`ActorComponent.ComponentHasTag` OtherComp "P")
    (goto _label)))

(event `self.WestDoor.OnComponentEndOverlap`
  (params (OverlappedComponent :type "PrimitiveComponent Object Reference") (OtherActor :type "Actor Object Reference") (OtherComp :type "PrimitiveComponent Object Reference") (OtherBodyIndex :type Integer))
  (if (`ActorComponent.ComponentHasTag` OtherComp "P")
    (`/Game/Blueprints/BP_MazeGen.ShowRoomC` (`/Game/Blueprints/Props/BP_Tile.Genrator` (`self.As BP Tile`)) :!label _label_2)))

(event `self.SouthDoor.OnComponentEndOverlap`
  (params (OverlappedComponent :type "PrimitiveComponent Object Reference") (OtherActor :type "Actor Object Reference") (OtherComp :type "PrimitiveComponent Object Reference") (OtherBodyIndex :type Integer))
  (if (`ActorComponent.ComponentHasTag` OtherComp "P")
    (goto _label_2)))

(event `self.EastDoor.OnComponentEndOverlap`
  (params (OverlappedComponent :type "PrimitiveComponent Object Reference") (OtherActor :type "Actor Object Reference") (OtherComp :type "PrimitiveComponent Object Reference") (OtherBodyIndex :type Integer))
  (if (`ActorComponent.ComponentHasTag` OtherComp "P")
    (goto _label_2)))

(event `self.NorthDoor.OnComponentEndOverlap`
  (params (OverlappedComponent :type "PrimitiveComponent Object Reference") (OtherActor :type "Actor Object Reference") (OtherComp :type "PrimitiveComponent Object Reference") (OtherBodyIndex :type Integer))
  (if (`ActorComponent.ComponentHasTag` OtherComp "P")
    (goto _label_2)))

(event `/Game/Blueprints/BI/BI_MazeComs.HideC`
  (set `self.Hidden` true)
  (bind (_direction _newtrack_0) (`Timeline|Timeline` :!label _label_3)
    (:`Update`
      (`SceneComponent.SetWorldScale3D` (`self.Ceiling`) (`KismetMathLibrary.VLerp` (1.0 1.0 1.0) (0.0 0.0 1.0) _newtrack_0)))
    (:`Finished`
      (`SceneComponent.SetHiddenInGame` (`self.Ceiling`) (select `ETimelineDirection` _direction :`Forward` true) false))))

(event `ShowC_1`
  (set `self.Hidden` false)
  (`SceneComponent.SetHiddenInGame` (`self.Ceiling`) false false)
  (goto _label_3 :!via `Reverse`))

(fn `AddDoor`
  (params (directions :type "/Game/Blueprints/Enum/E_Direction Enum" :default "NewEnumerator0"))
  (returns (NoWall :type Boolean))
  (locals (`Wall No` :type Boolean))
  (bind _returnvalue (`KismetStringLibrary.Conv_StringToName` (`|GetEnumeratorNameAsString` directions)))
  (for _array_element (`self.WallArray`)
    (if (`ActorComponent.ComponentHasTag` _array_element _returnvalue)
      (if (or (not (`SceneComponent.IsVisible` _array_element)) (`SceneComponent.bHiddenInGame` _array_element))
        (set `local.Wall No` true)
        (else
          (`KismetArrayLibrary.Array_Add` (`ActorComponent.ComponentTags` _array_element) "Door")
          (`StaticMeshComponent.SetStaticMesh` _array_element (select `int` (`self.Wall Index`) :`0` "/Game/Assest/DungeonResourcePack/Content/StaticMesh/Combined_85A19F8D.Combined_85A19F8D" :`1` "/Game/Assest/DungeonResourcePack/Content/StaticMesh/Combined_B910008B.Combined_B910008B" :`2` "/Game/Assest/DungeonResourcePack/Content/StaticMesh/Combined_0ECC570F.Combined_0ECC570F" :`3` "/Game/Assest/DungeonResourcePack/Content/StaticMesh/Combined_B910008B.Combined_B910008B" :`4` "/Game/Assest/DungeonResourcePack/Content/StaticMesh/Combined_CF22F982.Combined_CF22F982" :!type "StaticMesh Object Reference"))
          (for _array_element_2 (`SceneComponent.GetChildrenComponents` _array_element false)
            (bind _asbox_collision (cast `BoxComponent` _array_element_2))
            (set `PrimitiveComponent.bGenerateOverlapEvents` true _asbox_collision))))))
  (if (not (`local.Wall No`))
    (for _array_element_3 (`self.Signs`)
      (if (`ActorComponent.ComponentHasTag` _array_element_3 _returnvalue)
        (`SceneComponent.SetHiddenInGame` _array_element_3 false false))))
  (return (`local.Wall No`)))

(fn `FindExit`
  (params (IncomeDire :type "/Game/Blueprints/Enum/E_Direction Enum" :default "NewEnumerator0"))
  (returns (Exit :type "/Game/Blueprints/Enum/E_Direction Enum"))
  (return "NewEnumerator0"))

(fn `HideWall`
  (bind _directions (`/Game/Blueprints/Props/BP_Tile.Directions` (`self.As BP Tile`)))
  (bind _keys (`BlueprintMapLibrary.Map_Keys` _directions))
  (for _array_element _keys
    (if (`BlueprintMapLibrary.Map_Find` _directions _array_element)
      (for _array_element_2 (`self.WallArray`)
        (if (`ActorComponent.ComponentHasTag` _array_element_2 (`KismetStringLibrary.Conv_StringToName` (`|GetEnumeratorNameAsString` _array_element)))
          (`SceneComponent.SetHiddenInGame` _array_element_2 true false)
          (`PrimitiveComponent.SetCollisionEnabled` _array_element_2 "NoCollision"))))))

(fn `NewExit`
  (returns (NoExit :type Boolean) (ExitDirections :type "/Game/Blueprints/Enum/E_Direction Enum"))
  (return false "NewEnumerator0"))

(fn `SetRoomsWall`
  (bind _directions (`/Game/Blueprints/Props/BP_Tile.Directions` (`self.As BP Tile`)))
  (bind _keys (`BlueprintMapLibrary.Map_Keys` _directions))
  (for _array_element _keys
    (for _array_element_2 (`self.WallArray`)
      (if (`ActorComponent.ComponentHasTag` _array_element_2 (`KismetStringLibrary.Conv_StringToName` (`|GetEnumeratorNameAsString` _array_element)))
        (bind _value (`BlueprintMapLibrary.Map_Find` _directions _array_element))
        (`SceneComponent.SetVisibility` _array_element_2 (not _value) false)
        (`SceneComponent.SetHiddenInGame` _array_element_2 _value false)
        (`PrimitiveComponent.SetCollisionEnabled` _array_element_2 (select `bool` _value :`false` "QueryAndPhysics" :`true` "NoCollision" :!type "ECollisionEnabled Enum"))))))

(fn `SwapWalls`
  (params (RoomIndex :type Integer) (WallIndex :type Integer))
  (bind _returnvalue (`KismetMathLibrary.RandomIntegerInRange` 0 2))
  (set `self.Room Index` RoomIndex)
  (set `self.Wall Index` WallIndex)
  (for _array_element (`self.WallArray`)
    (`StaticMeshComponent.SetStaticMesh` _array_element (select `int` (`local.WallIndex`) :`0` (select `int` _returnvalue :`0` "/Game/Assest/DungeonResourcePack/Content/StaticMesh/Combined_E25D62AB.Combined_E25D62AB" :`1` "/Game/Assest/DungeonResourcePack/Content/StaticMesh/Combined_5945EF0C.Combined_5945EF0C" :`2` "/Game/Assest/DungeonResourcePack/Content/StaticMesh/Combined_80EE3539.Combined_80EE3539" :!type "StaticMesh Object Reference") :`1` (select `int` _returnvalue :`0` "/Game/Assest/DungeonResourcePack/Content/StaticMesh/DungeonGeneratorUE5_Plane_002.DungeonGeneratorUE5_Plane_002" :`1` "/Game/Assest/DungeonResourcePack/Content/StaticMesh/Combined_91FA1F61.Combined_91FA1F61" :`2` "/Game/Assest/DungeonResourcePack/Content/StaticMesh/Combined_D00667FD.Combined_D00667FD" :!type "StaticMesh Object Reference") :`2` (select `int` _returnvalue :`0` "/Game/Assest/DungeonResourcePack/Content/StaticMesh/Combined_A6E5690C.Combined_A6E5690C" :`1` "/Game/Assest/DungeonResourcePack/Content/StaticMesh/Combined_00365AE6.Combined_00365AE6" :`2` "/Game/Assest/DungeonResourcePack/Content/StaticMesh/Combined_91DBEEBD.Combined_91DBEEBD" :!type "StaticMesh Object Reference") :`3` (select `int` _returnvalue :`0` "/Game/Assest/DungeonResourcePack/Content/StaticMesh/Combined_AF8958EE.Combined_AF8958EE" :`1` "/Game/Assest/DungeonResourcePack/Content/StaticMesh/Combined_3E694B49.Combined_3E694B49" :`2` "/Game/Assest/DungeonResourcePack/Content/StaticMesh/Combined_C366F395.Combined_C366F395" :!type "StaticMesh Object Reference") :`4` (select `int` _returnvalue :`0` "/Game/Assest/DungeonResourcePack/Content/StaticMesh/Combined_4124F1AE.Combined_4124F1AE" :`1` "/Game/Assest/DungeonResourcePack/Content/StaticMesh/Combined_AEE127D0.Combined_AEE127D0" :`2` "/Game/Assest/DungeonResourcePack/Content/StaticMesh/Combined_18B24746.Combined_18B24746" :!type "StaticMesh Object Reference"))))
  (`SceneComponent.SetVisibility` (`self.Ceiling`) true false)
  (`PrimitiveComponent.SetCollisionEnabled` (`self.Ceiling`) "NoCollision")
  (set `PrimitiveComponent.bGenerateOverlapEvents` true (`self.Box`)))

(fn `UserConstructionScript`
  (set `self.WallArray` (`|MakeArray` (`self.Wall_N`) (`self.Wall_S`) (`self.Wall_E`) (`self.Wall_W`)))
  (set `self.Signs` (`|MakeArray` (`self.DoorSignE`) (`self.DoorSignW`) (`self.DoorSignS`) (`self.DoorSignN`)))
  (set `self.Torches` (`|MakeArray` (`self.SWR`) (`self.NWR`) (`self.NWL`) (`self.EWL`) (`self.EWR`) (`self.WWL`) (`self.WWR`) (`self.SWL`))))