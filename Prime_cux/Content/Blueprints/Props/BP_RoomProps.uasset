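; Dungeon-room prop dresser that decorates a room from its Directions map of open sides and walls.
; A torch goes on a random wall, or is removed if none exist.
; The open-side count picks the layout: one randomly rotated mesh, random meshes against walls, or two physics crates when fully open.
; Wall layouts sometimes spawn an all-open copy of itself for extra crates, with a destroy handler for cleanup.
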(event `self.ReceiveBeginPlay`
  (bind _staticmesha (`self.StaticMeshA`))
  (bind _values (`BlueprintMapLibrary.Map_Values` (`self.Directions`)))
  (for (_array_element _array_index) _values
    (if _array_element
      (set `self.NumberOfEmpty` (+ (`self.NumberOfEmpty`) 1))
      (else
        (`KismetArrayLibrary.Array_Add` (`self.Walls`) _array_index))))
  (`|ExecutionSequence`
    (:`then_0`
      (if (> (`KismetArrayLibrary.Array_Length` (`self.Walls`)) 0)
        (bind _keys (`BlueprintMapLibrary.Map_Keys` (`self.Directions`)))
        (bind _output (`|GetArrayItem` _keys (`KismetArrayLibrary.Array_Random` (`self.Walls`))))
        (set `self.RandomDirection` _output)
        (`SceneComponent.K2_SetRelativeLocation` (`self.RoomTorch`) (select `/Game/Blueprints/Enum/E_Direction` _output :`NewEnumerator0` (340.0 300.0 250.0) :`NewEnumerator1` (-340.0 300.0 250.0) :`NewEnumerator2` (-300.0 340.0 250.0) :`NewEnumerator3` (-300.0 -340.0 250.0) :!type "Vector Structure") false false)
        (`SceneComponent.K2_SetRelativeRotation` (`self.RoomTorch`) (select `/Game/Blueprints/Enum/E_Direction` _output :`NewEnumerator0` (struct :`Yaw` 90.0) :`NewEnumerator1` (struct :`Yaw` -90.0) :`NewEnumerator2` (struct :`Yaw` 180.0) :!type "Rotator Structure") false false)
        (else
          (`ActorComponent.K2_DestroyComponent` (`self.RoomTorch`)))))
    (:`then_1`
      (switch `int` (`self.NumberOfEmpty`)
        (:`1`
          (`ActorComponent.K2_DestroyComponent` (`self.StaticMeshB`))
          (`StaticMeshComponent.SetStaticMesh` _staticmesha (select `int` (`KismetMathLibrary.RandomIntegerInRange` 0 5) :`0` "/Game/Assest/DungeonResourcePack/Content/StaticMesh/Combined_16C54737.Combined_16C54737" :`1` "/Game/Assest/DungeonResourcePack/Content/StaticMesh/Combined_16C54737.Combined_16C54737" :`2` "/Game/Assest/DungeonResourcePack/Content/StaticMesh/Combined_85F1C003.Combined_85F1C003" :`3` "/Game/Assest/DungeonResourcePack/Content/StaticMesh/Combined_A8FCB639.Combined_A8FCB639" :`4` "/Game/Assest/DungeonResourcePack/Content/StaticMesh/Combined_A8FCB639.Combined_A8FCB639" :`5` "/Game/Assest/DungeonResourcePack/Content/StaticMesh/Combined_A8FCB639.Combined_A8FCB639" :!type "StaticMesh Object Reference"))
          (`SceneComponent.K2_SetRelativeRotation` _staticmesha (`KismetMathLibrary.MakeRotator` 0.0 0.0 (`KismetMathLibrary.RandomFloatInRange` 0.0 360.0)) false false)
          (`KismetSystemLibrary.PrintString` "1" true true (struct :`G` 0.66 :`B` 1.0 :`A` 1.0) 30.0))
        (:`2`
          (bind _keys_2 (`BlueprintMapLibrary.Map_Keys` (`self.Directions`)))
          (for (_array_element_2 _array_index_2) (`self.Walls`) :!label _label
            (bind _returnvalue (select `int` _array_index_2 :`0` (`self.StaticMeshA`) :`1` (`self.StaticMeshB`)))
            (`StaticMeshComponent.SetStaticMesh` _returnvalue (select `int` (`KismetMathLibrary.RandomIntegerInRange` 0 5) :`0` "/Game/Assest/DungeonResourcePack/Content/StaticMesh/Combined_85F1C003.Combined_85F1C003" :`1` "/Game/Assest/DungeonResourcePack/Content/StaticMesh/Combined_A8FCB639.Combined_A8FCB639" :`2` "/Game/Assest/DungeonResourcePack/Content/StaticMesh/Combined_16C54737.Combined_16C54737" :`3` "/Game/Assest/DungeonResourcePack/Content/StaticMesh/Combined_110F4126.Combined_110F4126" :`4` "/Game/Assest/DungeonResourcePack/Content/StaticMesh/Combined_85F1C003.Combined_85F1C003" :`5` "/Game/Assest/DungeonResourcePack/Content/StaticMesh/Combined_8E0425AA.Combined_8E0425AA" :!type "StaticMesh Object Reference"))
            (bind _output_2 (`|GetArrayItem` _keys_2 _array_element_2))
            (`SceneComponent.K2_SetRelativeLocation` _returnvalue (select `/Game/Blueprints/Enum/E_Direction` _output_2 :`NewEnumerator0` (350.0 0.0 0.0) :`NewEnumerator1` (-350.0 0.0 0.0) :`NewEnumerator2` (0.0 350.0 0.0) :`NewEnumerator3` (0.0 -350.0 0.0) :!type "Vector Structure") false false)
            (`SceneComponent.K2_SetRelativeRotation` _returnvalue (select `/Game/Blueprints/Enum/E_Direction` _output_2 :`NewEnumerator0` (struct :`Yaw` -90.0) :`NewEnumerator1` (struct :`Yaw` 90.0) :`NewEnumerator3` (struct :`Yaw` 180.0) :!type "Rotator Structure") false false)
            (`KismetSystemLibrary.PrintString` "Hello" true true (struct :`G` 0.66 :`B` 1.0 :`A` 1.0) 30.0))
          (switch `int` (`KismetMathLibrary.RandomIntegerInRange` 0 9)
            (:`0`
              _)
            (:`1`
              _)
            (:`2`
              _))
          (bind _returnvalue_2 (`|SpawnActorFromClass` "BP_RoomProps_C" (`KismetMathLibrary.MakeTransform` (`self.K2_GetActorLocation`)) "Undefined" "MultiplyWithRoot" null (`|MakeMap` "NewEnumerator0" true "NewEnumerator2" true "NewEnumerator1" true "NewEnumerator3" true :!type "/Game/Blueprints/Enum/E_Direction Enum") null))
          (add `self.OnDestroyed` (delegate `Destroy`)))
        (:`3`
          (`ActorComponent.K2_DestroyComponent` (`self.StaticMeshB`))
          (goto _label))
        (:`4`
          (for _array_element_3 (`|MakeArray` (`self.StaticMeshA`) (`self.StaticMeshB`))
            (`StaticMeshComponent.SetStaticMesh` _array_element_3 "/Game/Assest/DungeonResourcePack/Content/StaticMesh/PropItems_Square_Crate_Cube_001.PropItems_Square_Crate_Cube_001")
            (`SceneComponent.K2_SetWorldLocation` _array_element_3 (`KismetMathLibrary.RandomPointInBoundingBox` (+ (`self.K2_GetActorLocation`) (0.0 0.0 20.0)) (40.0 40.0 1.0)) false false)
            (set `PrimitiveComponent.CanCharacterStepUpOn` "ECB_No" _array_element_3)
            (set `ActorComponent.ComponentTags` (`|MakeArray` "PH" :!type "Name") _array_element_3)
            (`PrimitiveComponent.SetSimulatePhysics` _array_element_3 true)))))))

(event `Destroy` :!signature `self.OnDestroyed`
  (params (DestroyedActor :type "Actor Object Reference"))
  (`self.K2_DestroyActor` (stale `self.ReceiveBeginPlay` _returnvalue_2)))

(fn `UserConstructionScript`)