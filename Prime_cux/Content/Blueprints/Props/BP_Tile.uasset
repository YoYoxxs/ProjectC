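; Tile prop that tracks its open directions and picks random exits, apparently as a piece of a generated path.
; FindExit opens the side opposite the incoming direction plus a random exit, while NewExit opens another remaining exit or reports none left.
; Both consume a PossibleExits map and refresh arrow visibility from the Directions map.
; Construction labels the tile number and collects plant components; an event hides label and arrows in game.
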(event `HideAllArrows`
  (`SceneComponent.SetHiddenInGame` (`self.T_TileNumber`) true true)
  (`SceneComponent.SetHiddenInGame` (`self.ArrowNorth`) true true)
  (`SceneComponent.SetHiddenInGame` (`self.ArrowSouth`) true true)
  (`SceneComponent.SetHiddenInGame` (`self.ArrowEast`) true true)
  (`SceneComponent.SetHiddenInGame` (`self.ArrowWest`) true true))

(fn `FindExit`
  (params (IncomeDire :type "/Game/Blueprints/Enum/E_Direction Enum" :default "NewEnumerator0"))
  (returns (Exit :type "/Game/Blueprints/Enum/E_Direction Enum"))
  (bind _possibleexits (`self.PossibleExits`))
  (bind _value (`BlueprintMapLibrary.Map_Find` (`self.OpisiteDirection`) (`self.Income Dire`)))
  (set `self.Income Dire` IncomeDire)
  (`BlueprintMapLibrary.Map_Add` (`self.Directions`) _value true)
  (`BlueprintMapLibrary.Map_Remove` _possibleexits _value)
  (bind _keys (`BlueprintMapLibrary.Map_Keys` _possibleexits))
  (bind _output_get (set `self.Exit` (`KismetArrayLibrary.Array_Random` _keys)))
  (`BlueprintMapLibrary.Map_Remove` (`self.PossibleExits`) _output_get)
  (`BlueprintMapLibrary.Map_Add` (`self.Directions`) (`self.Exit`) true)
  (`self.ToggleArrows`)
  (return (`self.Exit`)))

(fn `NewExit`
  (returns (NoExit :type Boolean) (ExitDirections :type "/Game/Blueprints/Enum/E_Direction Enum"))
  (bind _possibleexits (`self.PossibleExits`))
  (bind _exit (`self.Exit`))
  (if (== (`BlueprintMapLibrary.Map_Length` _possibleexits) 0)
    (`/Game/Blueprints/BI/BI_MazeComs.ToggleArrows`)
    (return true "NewEnumerator0")
    (else
      (bind _keys (`BlueprintMapLibrary.Map_Keys` _possibleexits))
      (bind _output_get (set `self.Exit` (`KismetArrayLibrary.Array_Random` _keys)))
      (`BlueprintMapLibrary.Map_Add` (`self.Directions`) _output_get true)
      (`BlueprintMapLibrary.Map_Remove` (`self.PossibleExits`) _exit)
      (`/Game/Blueprints/BI/BI_MazeComs.ToggleArrows`)
      (return false _exit))))

(fn `ToggleArrows`
  (bind _keys (`BlueprintMapLibrary.Map_Keys` (`self.Directions`)))
  (for _array_element _keys
    (`SceneComponent.SetVisibility` (select `/Game/Blueprints/Enum/E_Direction` _array_element :`NewEnumerator0` (`self.ArrowNorth`) :`NewEnumerator1` (`self.ArrowSouth`) :`NewEnumerator2` (`self.ArrowEast`) :`NewEnumerator3` (`self.ArrowWest`)) (`BlueprintMapLibrary.Map_Find` (`self.Directions`) _array_element) true))
  (return))

(fn `UserConstructionScript`
  (`TextRenderComponent.K2_SetText` (`self.T_TileNumber`) (`KismetTextLibrary.Conv_StringToText` (`KismetStringLibrary.Concat_StrStr` "Tile Number Is:" (`KismetStringLibrary.Conv_IntToString` (`self.TileNumber`)))))
  (`self.ToggleArrows`)
  (set `self.Plants` (`|MakeArray` (`self.Plant1`) (`self.Plant3`) (`self.Plant2`) (`self.Plant`))))