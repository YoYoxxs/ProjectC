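; Elevator prop that carries the game from one generated maze level to the next, unlocked with inventory item I6.
; A tagged overlap consumes the item, spins the detached mechanism, spawns a higher-level BP_MazeGen above and blends the view to the elevator.
; A Timeline drives the fences, then Tick moves the actor up toward an externally controlled MaxAlpha point, returning the view to the pawn at the top.
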(event `self.ReceiveBeginPlay`
  (bind (_relativelocation_x _relativelocation_y _relativelocation_z) (`KismetMathLibrary.BreakVector` (`SceneComponent.RelativeLocation` (`self.Fence1`))))
  (set `self.OrignialFenceZ` _relativelocation_z)
  (bind _output_get (set `self.OriginalActorLocation` (`self.K2_GetActorLocation`)))
  (set `self.TargetActorLocation` (+ _output_get (0.0 0.0 2900.0))))

(event `self.ReceiveTick`
  (params (DeltaSeconds :type "Float (single-precision)"))
  (bind _returnvalue (`GameplayStatics.GetPlayerController` 0))
  (if (`self.TickCondition`)
    (`self.K2_SetActorLocation` (`KismetMathLibrary.VInterpTo_Constant` (`self.K2_GetActorLocation`) (`KismetMathLibrary.VLerp` (`self.OriginalActorLocation`) (`self.TargetActorLocation`) (`self.MaxAlpha`)) DeltaSeconds 350.0))
    (if (== (`self.TargetActorLocation`) (`self.K2_GetActorLocation`) :`ErrorTolerance` 10.0)
      (set `self.TickCondition` false)
      (`PlayerController.SetViewTargetWithBlend` _returnvalue (`Controller.K2_GetPawn` _returnvalue) 3.0 "VTBlend_Linear" 52.0 false))))

(event `self.Box.OnComponentBeginOverlap`
  (params (OverlappedComponent :type "PrimitiveComponent Object Reference") (OtherActor :type "Actor Object Reference") (OtherComp :type "PrimitiveComponent Object Reference") (OtherBodyIndex :type Integer) (bFromSweep :type Boolean) (SweepResult :type "HitResult Structure (by ref)"))
  (bind _generator (`self.Generator`))
  (bind _asbp_wave_game_mode (cast `/Game/Blueprints/BP_WaveGameMode` (`GameplayStatics.GetGameMode`) :!pure true))
  (bind _childactor (`ChildActorComponent.ChildActor` (`self.ChildActor`)))
  (bind _mazesize (`/Game/Blueprints/BP_MazeGen.MazeSize` _generator))
  (bind _returnvalue (+ _mazesize 1))
  (bind _inventory (`/Game/Blueprints/BP_WaveGameMode.Inventory` _asbp_wave_game_mode))
  (bind _returnvalue_2 (+ (`/Game/Blueprints/BP_MazeGen.MaxTiles` _generator) (`KismetMathLibrary.RandomIntegerInRange` 1 (+ (`/Game/Blueprints/BP_MazeGen.GeneratorLevel` _generator) 1))))
  (if (`ActorComponent.ComponentHasTag` OtherComp "P")
    (if (`.ReturnValue` (`BlueprintMapLibrary.Map_Find` _inventory "I6"))
      (`/Engine/EditorBlueprintResources/StandardMacros.DoOnce` false
        (:`Completed`
          (`self.K2_DetachFromActor` _childactor "KeepWorld" "KeepWorld" "KeepWorld")
          (set `RotatingMovementComponent.RotationRate` (struct :`Pitch` -60.0) (`/Game/Blueprints/Props/BP_ElevatorMechanice.RotatingMovement` (cast `/Game/Blueprints/Props/BP_ElevatorMechanice` _childactor :!pure true)))
          (`BlueprintMapLibrary.Map_Remove` _inventory "I6")
          (`/Game/UI/Widgets/WG_Hud.UpdateInventory` (`/Game/Blueprints/BP_WaveGameMode.WGHud` _asbp_wave_game_mode) _inventory)
          (`GameplayStatics.PlaySound2D` "/Game/Assest/DungeonResourcePack/Content/Sounds/Elevator/S_ElevatorUnlock.S_ElevatorUnlock" 1.0 1.0 0.0 null null)
          (bind _output_get (set `self.NewCenter` (+ (`self.K2_GetActorLocation`) (0.0 0.0 2500.0))))
          (`|SpawnActorFromClass` "/Game/Blueprints/BP_MazeGen.BP_MazeGen_C" (`KismetMathLibrary.MakeTransform` _output_get) "Undefined" "MultiplyWithRoot" null true _returnvalue_2 600 (select `bool` (< _returnvalue_2 (* _returnvalue _returnvalue)) :`false` _mazesize :`true` _returnvalue) (+ (`/Game/Blueprints/BP_MazeGen.GeneratorLevel` _generator) 1) self null)
          (`|ExecutionSequence`
            (:`then_0`
              (`PlayerController.SetViewTargetWithBlend` (`GameplayStatics.GetPlayerController` 0) self 3.0 "VTBlend_Linear" 0.0 false))
            (:`then_1`
              (`self.StartAnimation`)
              (`KismetSystemLibrary.Delay` 2.0)
              (set `self.TickCondition` true)
              (bind _returnvalue_3 (`GameplayStatics.CreateSound2D` "/Game/Assest/DungeonResourcePack/Content/Sounds/Elevator/Elevator_Machine.Elevator_Machine" 1.0 1.0 0.0 null))
              (bind _output_get_2 (set `self.ElevatorSound` _returnvalue_3))
              (`AudioComponent.Play` _output_get_2 0.0)))))
      (else
        (`GameplayStatics.PlaySound2D` "/Game/Assest/DungeonResourcePack/Content/Sounds/Elevator/S_ElevatorFail.S_ElevatorFail" 1.0 1.0 0.0 null null)))))

(event `StartAnimation`
  (bind (_direction _newtrack_0) (`Timeline|Timeline`)
    (:`Update`
      (for _array_element (`|MakeArray` (`self.Fence1`) (`self.Fence2`) (`self.Fence3`) (`self.Fence4`))
        (bind (_relativelocation_x _relativelocation_y) (`KismetMathLibrary.BreakVector` (`SceneComponent.RelativeLocation` _array_element)))
        (`SceneComponent.K2_SetRelativeLocation` _array_element (`KismetMathLibrary.MakeVector` _relativelocation_x _relativelocation_y (`KismetMathLibrary.Lerp` 0.0 0.0 _newtrack_0)) false false)))))

(fn `UserConstructionScript`)