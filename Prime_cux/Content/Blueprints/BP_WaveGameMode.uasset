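; Game mode that shows the main menu on BeginPlay, with events for loading, HUD and death screens, and manages the item inventory.
; AddToInventory looks up DT_Items, stacks stackable items in an inventory map capped at four entries, and refreshes the HUD.
; Non-inventory items roll coins by dungeon level but only write them to a HUD tooltip.
; CreateWaveHUD and UpdateGold are empty stubs.
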(event `self.ReceiveBeginPlay`
  ;[1 1 1] Begim
  (`self.ShowMainMenu`))

(event `ShowMainMenu`
  ;[1 1 1] Widget
  (bind _returnvalue (`|CreateWidget` "/Game/UI/Menus/WB_MainMenu.WB_MainMenu_C"))
  (bind _output_get (set `self.WgMainMenu` _returnvalue))
  (`UserWidget.AddToViewport` _output_get 0)
  (set `PlayerController.bShowMouseCursor` true (`GameplayStatics.GetPlayerController` 0)))

(event `ShowLoading`
  ;[1 1 1] Widget
  (bind _returnvalue (`|CreateWidget` "/Game/UI/Menus/WG_LoadingScreen.WG_LoadingScreen_C"))
  (bind _output_get (set `self.WgLoading` _returnvalue))
  (`UserWidget.AddToViewport` _output_get 0)
  (set `PlayerController.bShowMouseCursor` true (`GameplayStatics.GetPlayerController` 0)))

(event `Show Player HUD`
  ;[1 1 1] Widget
  (bind _returnvalue (`|CreateWidget` "/Game/UI/Widgets/WG_Hud.WG_Hud_C" (`GameplayStatics.GetPlayerController` 0) null))
  (bind _output_get (set `self.WGHud` _returnvalue))
  (`UserWidget.AddToViewport` _output_get 0))

(event `ShowDeath`
  ;[1 1 1] Widget
  (bind _returnvalue (`|CreateWidget` "/Game/UI/Widgets/WG_Death.WG_Death_C" (`GameplayStatics.GetPlayerController` 0)))
  (`UserWidget.AddToViewport` _returnvalue 0))

(fn `AddToInventory`
  (params (RowName :type Name))
  (returns (Picked :type Boolean))
  (locals (TempData :type "/Game/Blueprints/Items/ST_Items Structure") (TempVariable :type Integer))
  (bind _wghud (`self.WGHud`))
  (bind (_tempdata_itemname _tempdata_mesh _tempdata_itemsound _tempdata_inventoryimage _tempdata_addinventory _tempdata_stackable _tempdata_amount) (break `/Game/Blueprints/Items/ST_Items` (`local.TempData`)))
  (bind _inventory (`self.Inventory`))
  (bind (_tempdata_itemname_2 _tempdata_mesh_2 _tempdata_itemsound_2 _tempdata_inventoryimage_2 _tempdata_addinventory_2 _tempdata_stackable_2 _tempdata_amount_2) (break `/Game/Blueprints/Items/ST_Items` (`local.TempData`)))
  (bind _returnvalue (`|GetDataTableRow` "/Game/Blueprints/Items/DT_Items.DT_Items" RowName)
    (:`then`
      (bind _output_get (set `local.TempData` _returnvalue))
      (if (`.AddInventory_16_CA04E245426C3FD2398801B6B1C5EA85` (break `/Game/Blueprints/Items/ST_Items` _output_get))
        (if (`BlueprintMapLibrary.Map_Contains` _inventory (`local.RowName`))
          (if _tempdata_stackable
            (bind _output_get_2 (set `local.TempVariable` (`BlueprintMapLibrary.Map_Find` (`self.Inventory`) (`local.RowName`))))
            (`BlueprintMapLibrary.Map_Add` (`self.Inventory`) (`local.RowName`) (+ _tempdata_amount _output_get_2))
            (else
              (return false)))
          (elif (<= (`BlueprintMapLibrary.Map_Length` _inventory) 3)
            (`BlueprintMapLibrary.Map_Add` (`self.Inventory`) (`local.RowName`) _tempdata_amount_2)
            (else
              (return false))))
        (else
          (bind _output_get_3 (set `self.Coins` (`KismetMathLibrary.RandomIntegerInRange` 1 (+ (`self.Dungeon Level`) 1))))
          (`Widget.SetToolTipText` (`/Game/UI/Widgets/WG_Hud.TextBlock_CollectedCoins` (`self.WGHud`)) (`KismetTextLibrary.Conv_IntToText` _output_get_3))))
      (`/Game/UI/Widgets/WG_Hud.UpdateInventory` _wghud (`self.Inventory`))
      (`/Game/UI/Widgets/WG_Hud.ItemPickup` _wghud _tempdata_inventoryimage_2)
      (return true))))

(fn `CreateWaveHUD`)

(fn `Update gold`)

(fn `UserConstructionScript`)