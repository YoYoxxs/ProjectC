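; BP_HellGate is a gate actor that reacts when an actor tagged "P" enters or leaves its trigger sphere.
; On BeginPlay, RotatingMovement is set to spin the first static mesh.
; Entering the sphere sets Fire, switches both meshes to an alternate sigil material and starts the player's action music.
; Leaving clears Fire and restores the base material; nothing in this graph reads Fire or stops the music.
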(event `self.ReceiveBeginPlay`
  (`MovementComponent.SetUpdatedComponent` (`self.RotatingMovement`) (`self.StaticMesh`)))

(event `self.Sphere.OnComponentBeginOverlap`
  (params (OverlappedComponent :type "PrimitiveComponent Object Reference") (OtherActor :type "Actor Object Reference") (OtherComp :type "PrimitiveComponent Object Reference") (OtherBodyIndex :type Integer) (bFromSweep :type Boolean) (SweepResult :type "HitResult Structure (by ref)"))
  (if (`self.ActorHasTag` OtherActor "P")
    (set `self.Fire` true)
    (`PrimitiveComponent.SetMaterial` (`self.StaticMesh`) 0 "/Game/Assest/DungeonResourcePack/Content/Materials/SigilMM_Inst3.SigilMM_Inst3")
    (`PrimitiveComponent.SetMaterial` (`self.StaticMesh1`) 0 "/Game/Assest/DungeonResourcePack/Content/Materials/SigilMM_Inst3.SigilMM_Inst3")
    (`/Game/Blueprints/BP_Player.PlayActionMusic` (cast `/Game/Blueprints/BP_Player` OtherActor :!pure true))))

(event `self.Sphere.OnComponentEndOverlap`
  (params (OverlappedComponent :type "PrimitiveComponent Object Reference") (OtherActor :type "Actor Object Reference") (OtherComp :type "PrimitiveComponent Object Reference") (OtherBodyIndex :type Integer))
  (if (`self.ActorHasTag` OtherActor "P")
    (set `self.Fire` false)
    (`PrimitiveComponent.SetMaterial` (`self.StaticMesh`) 0 "/Game/Assest/DungeonResourcePack/Content/Materials/SigilMM.SigilMM")
    (`PrimitiveComponent.SetMaterial` (`self.StaticMesh1`) 0 "/Game/Assest/DungeonResourcePack/Content/Materials/SigilMM.SigilMM")))

(fn `UserConstructionScript`)