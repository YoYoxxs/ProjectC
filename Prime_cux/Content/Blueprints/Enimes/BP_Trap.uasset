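; BP_Trap is a spike trap that fires when a component tagged "P" enters its box.
; After a short delay with sound cues, a timeline raises the spikes and damage is applied to the player pawn if still overlapping.
; A Triggered flag blocks refiring until the timeline finishes in reverse through Revert, which nothing in this file calls.
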(event `self.ReceiveBeginPlay`
  (set `self.Relative Location` (`SceneComponent.RelativeLocation` (`self.Spikes`))))

(event `self.Box.OnComponentBeginOverlap`
  (params (OverlappedComponent :type "PrimitiveComponent Object Reference") (OtherActor :type "Actor Object Reference") (OtherComp :type "PrimitiveComponent Object Reference") (OtherBodyIndex :type Integer) (bFromSweep :type Boolean) (SweepResult :type "HitResult Structure (by ref)"))
  (if (and (`ActorComponent.ComponentHasTag` OtherComp "P") (not (`self.Triggered`)))
    (set `self.Triggered` true)
    (`GameplayStatics.PlaySound2D` "/Game/Assest/DungeonResourcePack/Content/Sounds/Trap/443806__deathscyp__spiketrap.443806__deathscyp__spiketrap" 1.0 1.0 0.0 null null)
    (`KismetSystemLibrary.Delay` 0.5)
    (`|ExecutionSequence`
      (:`then_0`
        (`GameplayStatics.PlaySound2D` "/Game/Assest/DungeonResourcePack/Content/Sounds/Trap/94121__bmaczero__mechanical2_Cue.94121__bmaczero__mechanical2_Cue" 1.0 1.0 0.0 null null))
      (:`then_1`
        (`self.Attack`)
        (for _array_element (`PrimitiveComponent.GetOverlappingActors` (`self.Box`) "/Game/Blueprints/BP_Player.BP_Player_C")
          (if (== (cast `/Game/Blueprints/BP_Player` _array_element :!pure true) (cast `/Game/Blueprints/BP_Player` (`GameplayStatics.GetPlayerPawn` 0) :!pure true))
            (`GameplayStatics.ApplyDamage` null 5.0)))
        (`KismetSystemLibrary.Delay` 0.5)))))

(event `Attack`
  (bind (_direction _newtrack_0) (`Timeline|Timeline` :!label _label)
    (:`Update`
      (`SceneComponent.K2_SetRelativeLocation` (`self.Spikes`) (`KismetMathLibrary.VLerp` (`self.Relative Location`) (0.0 0.0 30.0) _newtrack_0) false false))
    (:`Finished`
      (switch `ETimelineDirection` _direction
        (:`Backward`
          (set `self.Triggered` false))))))

(event `Revert`
  (goto _label :!via `ReverseFromEnd`))

(fn `UserConstructionScript`)