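; BP_Decorations is a child actor of BP_Tile that dresses a dungeon tile with four walls and a ceiling.
; HideWall and SetRoomsWall read the parent's Directions map, matching wall component tags to direction names to open or close sides, including collision.
; SwapWalls gives each wall a random mesh variant from the set chosen by WallIndex, then enables the ceiling and the Box's overlap events.
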(event `self.ReceiveBeginPlay`
  (bind _asbp_tile (cast `/Game/Blueprints/BP_Tile` (`self.GetParentActor`)))
  (set `self.As BP Tile` _asbp_tile))

(fn `HideWall`
  (bind _directions (`/Game/Blueprints/BP_Tile.Directions` (`self.As BP Tile`)))
  (bind _keys (`BlueprintMapLibrary.Map_Keys` _directions))
  (for _array_element _keys
    (if (`BlueprintMapLibrary.Map_Find` _directions _array_element)
      (for _array_element_2 (`self.WallArray`)
        (if (`ActorComponent.ComponentHasTag` _array_element_2 (`KismetStringLibrary.Conv_StringToName` (`|GetEnumeratorNameAsString` _array_element)))
          (`SceneComponent.SetHiddenInGame` _array_element_2 true false)
          (`PrimitiveComponent.SetCollisionEnabled` _array_element_2 "NoCollision"))))))

(fn `SetRoomsWall`
  (bind _directions (`/Game/Blueprints/BP_Tile.Directions` (`self.As BP Tile`)))
  (bind _keys (`BlueprintMapLibrary.Map_Keys` _directions))
  (for _array_element _keys
    (for _array_element_2 (`self.WallArray`)
      (if (`ActorComponent.ComponentHasTag` _array_element_2 (`KismetStringLibrary.Conv_StringToName` (`|GetEnumeratorNameAsString` _array_element)))
        (bind _value (`BlueprintMapLibrary.Map_Find` _directions _array_element))
        (`SceneComponent.SetVisibility` _array_element_2 (not _value) false)
        (`SceneComponent.SetHiddenInGame` _array_element_2 _value false)
        (`PrimitiveComponent.SetCollisionEnabled` _array_element_2 (select `bool` _value :`false` "QueryAndPhysics" :`true` "NoCollision" :!type "ECollisionEnabled Enum"))))))

(fn `SwapWalls`
  (params (RoomIndex :type Integer) (WallIndex :type Integer))
  (bind _returnvalue (`KismetMathLibrary.RandomIntegerInRange` 0 2))
  (set `self.Room Index` RoomIndex)
  (for _array_element (`self.WallArray`)
    (`StaticMeshComponent.SetStaticMesh` _array_element (select `int` (`local.WallIndex`) :`0` (select `int` _returnvalue :`0` "/Game/Assest/DungeonResourcePack/Content/StaticMesh/Combined_E25D62AB.Combined_E25D62AB" :`1` "/Game/Assest/DungeonResourcePack/Content/StaticMesh/Combined_5945EF0C.Combined_5945EF0C" :`2` "/Game/Assest/DungeonResourcePack/Content/StaticMesh/Combined_80EE3539.Combined_80EE3539" :!type "StaticMesh Object Reference") :`1` (select `int` _returnvalue :`0` "/Game/Assest/DungeonResourcePack/Content/StaticMesh/DungeonGeneratorUE5_Plane_002.DungeonGeneratorUE5_Plane_002" :`1` "/Game/Assest/DungeonResourcePack/Content/StaticMesh/Combined_91FA1F61.Combined_91FA1F61" :`2` "/Game/Assest/DungeonResourcePack/Content/StaticMesh/Combined_D00667FD.Combined_D00667FD" :!type "StaticMesh Object Reference") :`2` (select `int` _returnvalue :`0` "/Game/Assest/DungeonResourcePack/Content/StaticMesh/Combined_A6E5690C.Combined_A6E5690C" :`1` "/Game/Assest/DungeonResourcePack/Content/StaticMesh/Combined_00365AE6.Combined_00365AE6" :`2` "/Game/Assest/DungeonResourcePack/Content/StaticMesh/Combined_91DBEEBD.Combined_91DBEEBD" :!type "StaticMesh Object Reference") :`3` (select `int` _returnvalue :`0` "/Game/Assest/DungeonResourcePack/Content/StaticMesh/Combined_AF8958EE.Combined_AF8958EE" :`1` "/Game/Assest/DungeonResourcePack/Content/StaticMesh/Combined_3E694B49.Combined_3E694B49" :`2` "/Game/Assest/DungeonResourcePack/Content/StaticMesh/Combined_C366F395.Combined_C366F395" :!type "StaticMesh Object Reference") :`4` (select `int` _returnvalue :`0` "/Game/Assest/DungeonResourcePack/Content/StaticMesh/Combined_4124F1AE.Combined_4124F1AE" :`1` "/Game/Assest/DungeonResourcePack/Content/StaticMesh/Combined_AEE127D0.Combined_AEE127D0" :`2` "/Game/Assest/DungeonResourcePack/Content/StaticMesh/Combined_18B24746.Combined_18B24746" :!type "StaticMesh Object Reference"))))
  (`SceneComponent.SetVisibility` (`self.Ceiling`) true false)
  (`PrimitiveComponent.SetCollisionEnabled` (`self.Ceiling`) "QueryAndPhysics")
  (set `PrimitiveComponent.bGenerateOverlapEvents` true (`self.Box`)))

(fn `UserConstructionScript`
  (set `self.WallArray` (`|MakeArray` (`self.Wall_N`) (`self.Wall_S`) (`self.Wall_E`) (`self.Wall_W`))))