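; BP_AOE_OverTime_Base is a base Blueprint for area-of-effect abilities that act over time, extending its parent's Trigger event.
; Trigger calls the parent, then starts a looping timer at SpawnInterval and a second, non-looping timer set to Duration.
; The looping timer's delegate comes from a Create Event node with no visible target, and the Duration timer shows no bound event.
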(event `self.Trigger`
  (`parent.Trigger`)
  (`|ExecutionSequence`
    (:`then_0`
      (`KismetSystemLibrary.K2_SetTimerDelegate` (`|CreateDelegate` :!event `SpawnAOE`) (`self.SpawnInterval`) true))
    (:`then_1`
      (`KismetSystemLibrary.K2_SetTimerDelegate` :`Time` (`self.Duration`)))))

(fn `UserConstructionScript`
  (`parent.UserConstructionScript`))