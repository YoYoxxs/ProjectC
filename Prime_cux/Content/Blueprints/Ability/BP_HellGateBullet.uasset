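; Hell Gate bullet actor that flies at the player and explodes.
; On BeginPlay it randomly targets either the player pawn's location or a random point in a flat box below it.
; A timeline lerps it there, with a second track adding vertical offset to the target, then spawns an explosion and destroys it.
; Overlapping a component tagged "P" first applies slight damage, explodes and destroys it early.
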(event `self.ReceiveBeginPlay`
  (bind _returnvalue (`self.K2_GetActorLocation` (`GameplayStatics.GetPlayerPawn` 0)))
  (set `self.Target` (`KismetMathLibrary.SelectVector` (`KismetMathLibrary.RandomPointInBoundingBox` (- _returnvalue (0.0 0.0 100.0)) (200.0 200.0 1.0)) _returnvalue (`KismetMathLibrary.RandomBool`)))
  (set `self.OrignalLocation` (`self.K2_GetActorLocation`))
  (bind (_direction _newtrack_0 _newtrack_1) (`Timeline|Timeline`)
    (:`Update`
      (`self.K2_SetActorLocation` (`KismetMathLibrary.VLerp` (`self.OrignalLocation`) (+ (`self.Target`) (`KismetMathLibrary.VLerp` (0.0 0.0 0.0) (0.0 0.0 100.0) _newtrack_1)) _newtrack_0)))
    (:`Finished`
      (`GameplayStatics.SpawnEmitterAtLocation` "/Game/StarterContent/Particles/P_Explosion.P_Explosion" (`self.Target`) (struct) (0.5 0.5 0.5))
      (`self.K2_DestroyActor`))))

(event `self.Sphere.OnComponentBeginOverlap`
  (params (OverlappedComponent :type "PrimitiveComponent Object Reference") (OtherActor :type "Actor Object Reference") (OtherComp :type "PrimitiveComponent Object Reference") (OtherBodyIndex :type Integer) (bFromSweep :type Boolean) (SweepResult :type "HitResult Structure (by ref)"))
  (if (`ActorComponent.ComponentHasTag` OtherComp "P")
    (`GameplayStatics.ApplyDamage` OtherActor 0.1)
    (`GameplayStatics.SpawnEmitterAtLocation` "/Game/StarterContent/Particles/P_Explosion.P_Explosion" (`.Location` (`GameplayStatics.BreakHitResult` SweepResult)))
    (`self.K2_DestroyActor`)))

(fn `UserConstructionScript`)