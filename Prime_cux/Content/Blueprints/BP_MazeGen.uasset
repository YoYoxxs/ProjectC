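; Procedural maze generator that spawns a bounded grid dungeon of BP_Tile actors at BeginPlay while updating the game mode's loading bar.
; A delayed, recursive Build grows a snake path through empty neighbours, jumping back to random tiles at dead ends.
; It then reconciles exits between neighbours and places an elevator on the last tile and a chest near the middle.
; Finally, it carves non-overlapping 2x2 rooms with randomised internal walls.
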(event `self.ReceiveBeginPlay`
  (bind _as_bp_wave_game_mode (`self.As BP Wave Game Mode`))
  ;[0 0.1851 1] Begin
  (set `self.As BP Wave Game Mode` (cast `/Game/Blueprints/BP_WaveGameMode` (`GameplayStatics.GetGameMode`) :!pure true))
  (if (not (`self.Continue`))
    (`/Game/Blueprints/BP_WaveGameMode.ShowLoading` _as_bp_wave_game_mode)
    (`ProgressBar.SetPercent` (`/Game/UI/Menus/WG_LoadingScreen.Loadingbar` (`/Game/Blueprints/BP_WaveGameMode.WgLoading` _as_bp_wave_game_mode)) (`self.CalcTileLoading`))
    (`self.SpawnFirstTile`)
    (`self.Build`)))

(event `Build`
  (bind (_value _returnvalue) (`BlueprintMapLibrary.Map_Find` (`self.GetEmptyAdjacent` (`self.CurrentCorrds`)) (`self.Last Exit`)))
  ;[1 1 1] BuildTheMaze/ Dungeon Spwaning The Maze Like Snake And BackTracking When It Cant Spawn  A Tile
  (if (== (`self.CurrentTiles`) (`self.MaxTiles`))
    (`self.FixArrowsVisiability`)
    (`self.FixFalseExit`)
    (`ProgressBar.SetPercent` (`/Game/UI/Menus/WG_LoadingScreen.Loadingbar` (`/Game/Blueprints/BP_WaveGameMode.WgLoading` (`self.As BP Wave Game Mode`))) 0.45)
    (`self.Decoration`)
    (else
      (`KismetSystemLibrary.Delay` 0.2)
      (`ProgressBar.SetPercent` (`/Game/UI/Menus/WG_LoadingScreen.Loadingbar` (`/Game/Blueprints/BP_WaveGameMode.WgLoading` (`self.As BP Wave Game Mode`))) (`self.CalcTileLoading`))
      (set `self.CurrentTiles` (+ (`self.CurrentTiles`) 1))
      (if _returnvalue :!label _label
        (bind _output_get (set `self.CurrentCorrds` _value))
        (bind _returnvalue_2 (`|SpawnActorFromClass` "/Game/Blueprints/BP_Tile.BP_Tile_C" (`KismetMathLibrary.MakeTransform` (`self.FindTileLocation` _output_get)) "Undefined" "MultiplyWithRoot" null (`self.CurrentTiles`) self null))
        (`KismetArrayLibrary.Array_Add` (`self.ActorToDestroy`) _returnvalue_2)
        (`BlueprintMapLibrary.Map_Add` (`self.DungeonMap`) (`self.CurrentCorrds`) _returnvalue_2)
        (bind _exit (message `/Game/Blueprints/BI/BI_MazeComs.FindExit` _returnvalue_2 (`self.Last Exit`)))
        (set `self.Last Exit` _exit)
        (`self.Build`)
        (else
          (bind _noexit (`self.TryToBackTrack` :!label _label_2))
          (if _noexit
            (if (== (`BlueprintMapLibrary.Map_Length` (`self.DungeonMap`)) (`BlueprintMapLibrary.Map_Length` (`self.VisitedLocation`)))
              (`KismetSystemLibrary.PrintString` "MazeCantBuildMore" true true (struct :`R` 1.0 :`G` 0.01368 :`A` 1.0) 10.0)
              (set `self.CurrentTiles` (`self.MaxTiles`))
              (`self.Build`)
              (else
                (goto _label_2)))
            (else
              (`self.ContiuneBuild`))))))))

(event `ContiuneBuild`
  ;[1 1 1] BuildTheMaze/ Dungeon Spwaning The Maze Like Snake And BackTracking When It Cant Spawn  A Tile
  (goto _label))

(event `Decoration`
  (`self.BasicLayout`)
  (`KismetSystemLibrary.Delay` 0.1)
  (`ProgressBar.SetPercent` (`/Game/UI/Menus/WG_LoadingScreen.Loadingbar` (`/Game/Blueprints/BP_WaveGameMode.WgLoading` (`self.As BP Wave Game Mode`))) 0.5)
  (`self.CreateCoordsElevator`)
  (`self.CreateCoordsChest`)
  (`self.FindPossiableRooms2x2`)
  (`self.BuildRooms`))

(fn `BasicLayout`
  (bind _values (`BlueprintMapLibrary.Map_Values` (`self.DungeonMap`)))
  (for _array_element _values
    (`/Game/Blueprints/BP_Decorations.HideWall` (cast `/Game/Blueprints/BP_Decorations` (`ChildActorComponent.ChildActor` (`/Game/Blueprints/BP_Tile.Decoration` _array_element)) :!pure true))))

(fn `BuildRooms`
  (locals (RoomIndex :type Integer) (WallIndex :type Integer) (InternalWallIndex :type Integer :default 0) (TileOfInternalWall :type "IntPoint Structure"))
  (bind _returnvalue (`KismetMathLibrary.RandomBool`))
  (bind _directions (`/Game/Blueprints/BP_Tile.Directions` (`BlueprintMapLibrary.Map_Find` (`self.DungeonMap`) (`local.TileOfInternalWall`))))
  (for (_array_element _array_index) (`self.STRoomsArry`)
    (bind _output_get (set `local.RoomIndex` _array_index))
    (if (> _output_get 2)
      (set `local.WallIndex` (`KismetMathLibrary.RandomIntegerInRange` 0 4))
      (else
        (set `local.WallIndex` (`local.RoomIndex`))))
    (set `local.InternalWallIndex` (`KismetMathLibrary.RandomIntegerInRange` 0 3))
    (bind _roomcoords (break `/Game/Blueprints/Structures/ST_Rooms` _array_element))
    (set `local.TileOfInternalWall` (`|GetArrayItem` _roomcoords (`local.InternalWallIndex`)))
    (for (_array_element_2 _array_index_2) _roomcoords
      (switch `int` _array_index_2
        (:`0`
          (bind _directions_2 (`/Game/Blueprints/BP_Tile.Directions` (`BlueprintMapLibrary.Map_Find` (`self.DungeonMap`) _array_element_2)))
          (`BlueprintMapLibrary.Map_Add` _directions_2 "NewEnumerator2" true)
          (`BlueprintMapLibrary.Map_Add` _directions_2 "NewEnumerator1" true)
          (`BlueprintMapLibrary.Map_Add` _directions_2 "NewEnumerator0")
          (`BlueprintMapLibrary.Map_Add` _directions_2 "NewEnumerator3"))
        (:`1`
          (`BlueprintMapLibrary.Map_Add` _directions_2 "NewEnumerator0" true)
          (`BlueprintMapLibrary.Map_Add` _directions_2 "NewEnumerator3" true)
          (`BlueprintMapLibrary.Map_Add` _directions_2 "NewEnumerator1")
          (`BlueprintMapLibrary.Map_Add` _directions_2 "NewEnumerator2"))
        (:`2`
          (`BlueprintMapLibrary.Map_Add` _directions_2 "NewEnumerator3" true)
          (`BlueprintMapLibrary.Map_Add` _directions_2 "NewEnumerator1" true)
          (`BlueprintMapLibrary.Map_Add` _directions_2 "NewEnumerator0")
          (`BlueprintMapLibrary.Map_Add` _directions_2 "NewEnumerator2"))
        (:`3`
          (`BlueprintMapLibrary.Map_Add` _directions_2 "NewEnumerator0" true)
          (`BlueprintMapLibrary.Map_Add` _directions_2 "NewEnumerator2" true)
          (`BlueprintMapLibrary.Map_Add` _directions_2 "NewEnumerator1")
          (`BlueprintMapLibrary.Map_Add` _directions_2 "NewEnumerator3"))))
    (switch `int` (`KismetMathLibrary.SelectInt` 4 (`local.InternalWallIndex`) (`KismetMathLibrary.RandomBool`))
      (:`0`
        (if _returnvalue
          (`BlueprintMapLibrary.Map_Add` _directions "NewEnumerator2")
          (else
            (`BlueprintMapLibrary.Map_Add` _directions "NewEnumerator1"))))
      (:`1`
        (if _returnvalue
          (`BlueprintMapLibrary.Map_Add` _directions "NewEnumerator0")
          (else
            (`BlueprintMapLibrary.Map_Add` _directions "NewEnumerator3"))))
      (:`2`
        (if _returnvalue
          (`BlueprintMapLibrary.Map_Add` _directions "NewEnumerator3")
          (else
            (`BlueprintMapLibrary.Map_Add` _directions "NewEnumerator1"))))
      (:`3`
        (if _returnvalue
          (`BlueprintMapLibrary.Map_Add` _directions "NewEnumerator0")
          (else
            (`BlueprintMapLibrary.Map_Add` _directions "NewEnumerator2"))))
      (:`4`
        _))
    (for _array_element_3 _roomcoords
      (bind _value (`BlueprintMapLibrary.Map_Find` (`self.DungeonMap`) _array_element_3))
      (message `/Game/Blueprints/BI/BI_MazeComs.ToggleArrows` _value)
      (`/Game/Blueprints/BP_Decorations.SetRoomsWall` (cast `/Game/Blueprints/BP_Decorations` (`ChildActorComponent.ChildActor` (`/Game/Blueprints/BP_Tile.Decoration` _value)) :!pure true)))))

(fn `CalcTileLoading`
  (returns (Percentage :type "Float (double-precision)"))
  (return (/ 40.0 (* (/ (`KismetMathLibrary.Conv_IntToDouble` (`self.MaxTiles`)) (`KismetMathLibrary.Conv_IntToDouble` (`self.CurrentTiles`))) 100.0))))

(fn `CheckIfOutOfBounds`
  (params (IntPoint :type "IntPoint Structure (by ref)"))
  (returns (OutOfBounds :type Boolean))
  (bind (_x _y) (break `IntPoint` IntPoint))
  (bind _mazesize (`self.MazeSize`))
  (bind _returnvalue (* (`self.MazeSize`) -1))
  (return (or (> _y _mazesize) (> _x _mazesize) (< _x _returnvalue) (< _y _returnvalue))))

(fn `CreateCoordsChest`
  (locals (ChestIndex :type Integer) (Trys :type Integer))
  (bind _trys (`local.Trys`))
  (bind _returnvalue (+ (`local.ChestIndex`) 1))
  (bind _keys (`BlueprintMapLibrary.Map_Keys` (`self.DungeonMap`)))
  (bind _returnvalue_2 (/ (`KismetArrayLibrary.Array_LastIndex` _keys) 2))
  (set `local.ChestIndex` _returnvalue_2)
  (while (== (`local.ChestIndex`) _returnvalue_2)
    (`/Engine/EditorBlueprintResources/StandardMacros.IncrementInt` _trys
      (:`  `
        (if (== _trys _returnvalue_2)
          (set `local.ChestIndex` 0)
          (elif (not (`KismetArrayLibrary.Array_Contains` (`self.SpecialTiles`) (`|GetArrayItem` _keys _returnvalue)))
            (set `local.ChestIndex` _returnvalue))))))
  (if (== (`local.ChestIndex`) 0)
    (set `local.ChestIndex` _returnvalue_2)
    (else
      (bind _output (`|GetArrayItem` _keys (`local.ChestIndex`)))
      (`KismetArrayLibrary.Array_Add` (`self.SpecialTiles`) _output)
      (set `self.ChestLocation` _output)
      (bind _returnvalue_3 (`|SpawnActorFromClass` "/Game/Blueprints/BP_BigChest.BP_BigChest_C" (`KismetMathLibrary.MakeTransform` (`self.K2_GetActorLocation` (`BlueprintMapLibrary.Map_Find` (`self.DungeonMap`) (`self.ChestLocation`)))) "Undefined" "MultiplyWithRoot" null null))
      (set `self.Chest spawn` _returnvalue_3))))

(fn `CreateCoordsElevator`
  (bind _keys (`BlueprintMapLibrary.Map_Keys` (`self.DungeonMap`)))
  (bind _output_get (set `self.ElevatorLocation` (`|GetArrayItem` _keys (`KismetArrayLibrary.Array_LastIndex` _keys))))
  (`KismetArrayLibrary.Array_Add` (`self.SpecialTiles`) _output_get)
  (for _array_element (`self.FindSingleTilePrimeter` (`self.ElevatorLocation`))
    (if (`BlueprintMapLibrary.Map_Contains` (`self.DungeonMap`) _array_element)
      (`KismetArrayLibrary.Array_Add` (`self.SpecialTiles`) _array_element)))
  (bind _returnvalue (`|SpawnActorFromClass` "/Game/Blueprints/BP_Elevator.BP_Elevator_C" (`KismetMathLibrary.MakeTransform` (`self.K2_GetActorLocation` (`BlueprintMapLibrary.Map_Find` (`self.DungeonMap`) (`self.ElevatorLocation`)))) "Undefined" "MultiplyWithRoot" null null))
  (set `self.SpawnedElevator` _returnvalue))

(fn `FindCrossAdjust`
  (params (Coords :type "IntPoint Structure"))
  (returns (Adjacent :type "Array of IntPoint Structure"))
  (bind (_x _y) (break `IntPoint` Coords))
  (return (`|MakeArray` (make `IntPoint` (+ _x 1) _y) (make `IntPoint` (- _x 1) _y) (make `IntPoint` _x (+ _y 1)) (make `IntPoint` _x (- _y 1)))))

(fn `FindPossiableRooms2x2`
  (locals (ValidRoom :type Boolean :default true) (RoomArry :type "Array of IntPoint Structure") (RoomST :type "/Game/Blueprints/Structures/ST_Rooms Structure"))
  (bind _roomarry (`local.RoomArry`))
  (bind _keys (`BlueprintMapLibrary.Map_Keys` (`self.DungeonMap`)))
  (for _array_element _keys
    (set `local.ValidRoom` true)
    (`KismetArrayLibrary.Array_Clear` (`local.RoomArry`))
    (for _array_element_2 (`self.Make2X2RoomCoords` _array_element)
      (if (`BlueprintMapLibrary.Map_Contains` (`self.DungeonMap`) _array_element_2)
        (`KismetArrayLibrary.Array_Add` (`local.RoomArry`) _array_element_2)
        (else
          (set `local.ValidRoom` false)
          (break))))
    (if (`local.ValidRoom`)
      (for _array_element_3 (`local.RoomArry`)
        (if (or (`KismetArrayLibrary.Array_Contains` (`self.SpecialTiles`) _array_element_3) (`KismetArrayLibrary.Array_Contains` (`self.AllRoomPremeter`) _array_element_3))
          (set `local.ValidRoom` false)
          (break)))
      (if (`local.ValidRoom`)
        (for _array_element_4 (`self.STRoomsArry`)
          (if (`local.ValidRoom`)
            (for _array_element_5 (`.RoomCoords_4_CDE73B6C4776FE51199B82B3DFA15F5F` (break `/Game/Blueprints/Structures/ST_Rooms` _array_element_4))
              (if (`KismetArrayLibrary.Array_Contains` (`local.RoomArry`) _array_element_5)
                (set `local.ValidRoom` false)
                (break)))
            (else
              (break))))
        (if (`local.ValidRoom`)
          (bind _structout (setmembers `/Game/Blueprints/Structures/ST_Rooms` :`StructRef` (`local.RoomST`) :`RoomCoords` _roomarry))
          (`KismetArrayLibrary.Array_Add` (`self.STRoomsArry`) _structout)
          (`self.SetRoomPremeter` _roomarry)))))
  (for _array_element_6 (`self.STRoomsArry`)
    (for _array_element_7 (`.RoomCoords_4_CDE73B6C4776FE51199B82B3DFA15F5F` (break `/Game/Blueprints/Structures/ST_Rooms` _array_element_6))
      (`KismetArrayLibrary.Array_Add` (`self.AllRoomCoords`) _array_element_7)
      (`PrimitiveComponent.SetMaterial` (`/Game/Blueprints/BP_Tile.Floor` (`BlueprintMapLibrary.Map_Find` (`self.DungeonMap`) _array_element_7)) 0 "/Game/Assest/DungeonResourcePack/Content/Materials/BrickWallDirty.BrickWallDirty"))))

(fn `FindRoomIndex`
  (params (Coords :type "IntPoint Structure"))
  (returns (FoundRoom :type Boolean) (RoomIndex :type Integer))
  (locals (RoomFound :type Boolean) (RoomNumber :type Integer))
  (for (_array_element _array_index) (`self.STRoomsArry`)
    (if (`KismetArrayLibrary.Array_Contains` (`.RoomCoords_4_CDE73B6C4776FE51199B82B3DFA15F5F` (break `/Game/Blueprints/Structures/ST_Rooms` _array_element)) Coords)
      (set `local.RoomFound` true)
      (set `local.RoomNumber` _array_index)
      (break)))
  (return (`local.RoomFound`) (`local.RoomNumber`)))

(fn `FindSingleTilePrimeter`
  (params (Coords :type "IntPoint Structure"))
  (returns (PremeterTileCoords :type "Array of IntPoint Structure"))
  (bind (_x _y) (break `IntPoint` Coords))
  (bind _returnvalue (+ _x 1))
  (bind _returnvalue_2 (- _x 1))
  (bind _returnvalue_3 (+ _y 1))
  (bind _returnvalue_4 (- _y 1))
  (return (`|MakeArray` (make `IntPoint` _returnvalue _y) (make `IntPoint` _returnvalue_2 _y) (make `IntPoint` _x _returnvalue_3) (make `IntPoint` _x _returnvalue_4) (make `IntPoint` _returnvalue _returnvalue_3) (make `IntPoint` _returnvalue _returnvalue_4) (make `IntPoint` _returnvalue_2 _returnvalue_3) (make `IntPoint` _returnvalue_2 _returnvalue_4))))

(fn `FindTileLocation`
  (params (Coords :type "IntPoint Structure"))
  (returns (Location :type "Vector Structure"))
  (bind (_x _y) (break `IntPoint` Coords))
  (bind _tilesize (`self.TileSize`))
  (return (+ (`KismetMathLibrary.MakeVector` (* _x _tilesize) (* _tilesize _y)) (`self.K2_GetActorLocation`))))

(fn `FixArrowsVisiability`
  (bind _keys (`BlueprintMapLibrary.Map_Keys` (`self.DungeonMap`)))
  (for _array_element _keys
    (bind _validadjacent1 (`self.GetFilledAdjecnt` _array_element))
    (bind _keys_2 (`BlueprintMapLibrary.Map_Keys` _validadjacent1))
    (for _array_element_2 _keys_2
      (bind _value (`BlueprintMapLibrary.Map_Find` (`self.DungeonMap`) (`BlueprintMapLibrary.Map_Find` _validadjacent1 _array_element_2)))
      (`BlueprintMapLibrary.Map_Add` (`/Game/Blueprints/BP_Tile.Directions` _value) (`BlueprintMapLibrary.Map_Find` (`/Game/Blueprints/BP_Tile.OpisiteDirection` _value) _array_element_2) (`BlueprintMapLibrary.Map_Find` (`/Game/Blueprints/BP_Tile.Directions` (`BlueprintMapLibrary.Map_Find` (`self.DungeonMap`) _array_element)) _array_element_2))
      (message `/Game/Blueprints/BI/BI_MazeComs.ToggleArrows` _value))))

(fn `FixFalseExit`
  (bind _dungeonmap (`self.DungeonMap`))
  (bind _keys (`BlueprintMapLibrary.Map_Keys` _dungeonmap))
  (for _array_element _keys
    (bind _value (`BlueprintMapLibrary.Map_Find` _dungeonmap _array_element))
    (bind _directions (`/Game/Blueprints/BP_Tile.Directions` _value))
    (bind _keys_2 (`BlueprintMapLibrary.Map_Keys` _directions))
    (for _array_element_2 _keys_2
      (if (not (`BlueprintMapLibrary.Map_Contains` (`self.GetFilledAdjecnt` _array_element) _array_element_2))
        (`BlueprintMapLibrary.Map_Add` _directions _array_element_2)
        (message `/Game/Blueprints/BI/BI_MazeComs.ToggleArrows` _value)))))

(fn `GetEmptyAdjacent`
  (params (Coords :type "IntPoint Structure"))
  (returns (VaildAdjacentValues :type "Map of /Game/Blueprints/Enum/E_Direction Enum to IntPoint Structure"))
  (locals (VaildAdjacent :type "Map of /Game/Blueprints/Enum/E_Direction Enum to IntPoint Structure"))
  (for (_array_element _array_index) (`self.FindCrossAdjust` Coords)
    (bind _keys (`BlueprintMapLibrary.Map_Keys` (`self.DungeonMap`)))
    (if (not (or (`KismetArrayLibrary.Array_Contains` _keys _array_element) (`KismetArrayLibrary.Array_Contains` (`self.ForcedEmpty`) _array_element) (`self.CheckIfOutOfBounds` _array_element)))
      (`BlueprintMapLibrary.Map_Add` (`local.VaildAdjacent`) (select `int` _array_index :`0` "NewEnumerator0" :`1` "NewEnumerator1" :`2` "NewEnumerator2" :`3` "NewEnumerator3" :!type "/Game/Blueprints/Enum/E_Direction Enum") _array_element)))
  (return (`local.VaildAdjacent`)))

(fn `GetFilledAdjecnt`
  (params (Coords :type "IntPoint Structure"))
  (returns (ValidAdjacent1 :type "Map of /Game/Blueprints/Enum/E_Direction Enum to IntPoint Structure"))
  (locals (ValidAdjacent :type "Map of /Game/Blueprints/Enum/E_Direction Enum to IntPoint Structure"))
  (for (_array_element _array_index) (`self.FindCrossAdjust` Coords)
    (if (`BlueprintMapLibrary.Map_Contains` (`self.DungeonMap`) _array_element)
      (`BlueprintMapLibrary.Map_Add` (`local.ValidAdjacent`) (select `int` _array_index :`0` "NewEnumerator0" :`1` "NewEnumerator1" :`2` "NewEnumerator2" :`3` "NewEnumerator3" :!type "/Game/Blueprints/Enum/E_Direction Enum") _array_element)))
  (return (`local.ValidAdjacent`)))

(fn `Make2X2RoomCoords`
  (params (Coords :type "IntPoint Structure"))
  (returns (RoomCoords :type "Array of IntPoint Structure"))
  (bind (_x _y) (break `IntPoint` Coords))
  (bind _returnvalue (+ _x 1))
  (bind _returnvalue_2 (+ _y 1))
  (return (`|MakeArray` (make `IntPoint` _returnvalue _y) (make `IntPoint` _x _returnvalue_2) (make `IntPoint` _returnvalue _returnvalue_2) Coords)))

(fn `SetRoomPremeter`
  (params (RoomsArray :type "Array of IntPoint Structure"))
  (locals (RoomPremeter :type "Array of IntPoint Structure"))
  (bind (_x _y) (break `IntPoint` (`|GetArrayItem` RoomsArray (`KismetArrayLibrary.Array_LastIndex` RoomsArray))))
  (for _index (range (- _x 1) (+ (+ _x 2) 1))
    (for _index_2 (range (- _y 1) (+ (+ _y 2) 1))
      (if (not (`KismetArrayLibrary.Array_Contains` (`local.RoomsArray`) (make `IntPoint` _index _index_2)))
        (`KismetArrayLibrary.Array_Add` (`local.RoomPremeter`) (make `IntPoint` _index _index_2))
        (`KismetArrayLibrary.Array_Add` (`self.AllRoomPremeter`) (make `IntPoint` _index _index_2)))))
  (for _array_element (`local.RoomPremeter`)
    (for (_array_element_2 _array_index) (`self.FindCrossAdjust` _array_element)
      (if (`self.FindRoomIndex` _array_element_2)
        (bind _value (`BlueprintMapLibrary.Map_Find` (`self.DungeonMap`) _array_element))
        (`/Engine/EditorBlueprintResources/StandardMacros.IsValid` _value
          (:`Is Valid`
            (for _array_element_3 (`self.K2_GetComponentsByClass` (cast `/Game/Blueprints/BP_Decorations` (`ChildActorComponent.ChildActor` (`/Game/Blueprints/BP_Tile.Decoration` _value)) :!pure true) "/Script/Engine.StaticMeshComponent")
              (if (`ActorComponent.ComponentHasTag` _array_element_3 (`KismetStringLibrary.Conv_StringToName` (`|GetEnumeratorNameAsString` (select `int` _array_index :`0` "NewEnumerator0" :`1` "NewEnumerator1" :`2` "NewEnumerator2" :`3` "NewEnumerator3" :!type "/Game/Blueprints/Enum/E_Direction Enum"))))
                (`SceneComponent.SetHiddenInGame` _array_element_3 true false)
                (`PrimitiveComponent.SetCollisionEnabled` _array_element_3 "NoCollision")))))))))

(fn `SpawnFirstTile`
  (bind _currentcorrds (`self.CurrentCorrds`))
  (if (not (`self.Continue`))
    (bind _returnvalue (`|SpawnActorFromClass` "/Game/Blueprints/BP_Tile.BP_Tile_C" (`KismetMathLibrary.MakeTransform` (`self.K2_GetActorLocation`)) "Undefined" "MultiplyWithRoot" null 0 self null))
    (`KismetArrayLibrary.Array_Add` (`self.ActorToDestroy`) _returnvalue)
    (`BlueprintMapLibrary.Map_Add` (`self.DungeonMap`) _currentcorrds _returnvalue)
    (`KismetArrayLibrary.Array_Add` (`self.SpecialTiles`) _currentcorrds)
    (bind _output_get (set `self.Last Exit` (`KismetArrayLibrary.Array_Random` (`|MakeArray` "NewEnumerator0" "NewEnumerator1" "NewEnumerator2" "NewEnumerator3" :!type "/Game/Blueprints/Enum/E_Direction Enum"))))
    (`BlueprintMapLibrary.Map_Add` (`/Game/Blueprints/BP_Tile.Directions` _returnvalue) _output_get true)
    (bind _output (`|GetArrayItem` (`self.FindCrossAdjust` _currentcorrds) (select `/Game/Blueprints/Enum/E_Direction` _output_get)))
    (`KismetArrayLibrary.Array_Add` (`self.ForcedEmpty`) _output)
    (bind _returnvalue_2 (`|SpawnActorFromClass` "/Game/Blueprints/BP_Intro.BP_Intro_C" (`KismetMathLibrary.MakeTransform` (+ (`self.FindTileLocation` _output) (0.0 0.0 300.0))) "Undefined" "MultiplyWithRoot" null null))
    (`KismetArrayLibrary.Array_Add` (`self.ActorToDestroy`) _returnvalue_2)))

(fn `TryToBackTrack`
  (returns (NoExit :type Boolean))
  (locals (RandomLocations :type Integer :default 0))
  (bind _keys (`BlueprintMapLibrary.Map_Keys` (`self.DungeonMap`)))
  (bind _output_get (set `local.RandomLocations` (`.OutIndex` (`KismetArrayLibrary.Array_Random` _keys))))
  (bind _output (`|GetArrayItem` _keys _output_get))
  (if (`BlueprintMapLibrary.Map_Contains` (`self.VisitedLocation`) _output)
    (return true)
    (else
      (bind _value (`BlueprintMapLibrary.Map_Find` (`self.DungeonMap`) _output))
      (`BlueprintMapLibrary.Map_Add` (`self.VisitedLocation`) _output _value)
      (bind (_noexit _exitdirections) (message `/Game/Blueprints/BI/BI_MazeComs.NewExit` _value))
      (if _noexit
        (return true)
        (else
          (set `self.Last Exit` _exitdirections)
          (set `self.CurrentCorrds` _output)
          (return false))))))

(fn `UserConstructionScript`)