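; BP_MouseInteraction handles cursor targeting and hover messages for interactable items.
; GetMouseLocation traces under the cursor, sphere-traces from the player camera to that point, and returns a location, falling back to a deprojected point far along the cursor ray.
; It tracks hovered actors tagged "I", sending start/end hover messages, while ClearItemSelect resets them.
; Right-click handlers only run validity checks, and the event graph's Interact call is unconnected.
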(event `self.ReceiveBeginPlay`
  (set `self.As BP Wave Game Mode` (cast `/Game/Blueprints/BP_WaveGameMode` (`GameplayStatics.GetGameMode`) :!pure true)))

(event `EnhancedInput|/Game/UI/Input/Actions/IA_RightClick`
  (params (ActionValue :type Boolean) (ElapsedSeconds :type "Float (double-precision)") (TriggeredSeconds :type "Float (double-precision)") (InputAction :type "InputAction Object Reference" :default "/Game/UI/Input/Actions/IA_RightClick.IA_RightClick"))
  (:`Triggered`
    (`/Engine/EditorBlueprintResources/StandardMacros.IsValid` (`self.CurrentItemTarget`)))
  (:`Completed`
    (`/Engine/EditorBlueprintResources/StandardMacros.IsValid` (`/Game/Blueprints/BP_WaveGameMode.As BP Player` (`self.As BP Wave Game Mode`))
      (:`Is Valid`
        (`/Engine/EditorBlueprintResources/StandardMacros.IsValid` (`self.CurrentItemTarget`))))))

(fn `ClearItemSelect`
  (bind _previtemtarget (`self.PrevItemTarget`))
  (bind _currentitemtarget (`self.CurrentItemTarget`))
  (`/Engine/EditorBlueprintResources/StandardMacros.IsValid` _previtemtarget
    (:`Is Valid`
      (message `/Game/Blueprints/BI/BI_ItemComponant.EndHover` _previtemtarget))
    (:`Is Not Valid`
      _))
  (`/Engine/EditorBlueprintResources/StandardMacros.IsValid` _currentitemtarget
    (:`Is Valid`
      (message `/Game/Blueprints/BI/BI_ItemComponant.EndHover` _currentitemtarget))
    (:`Is Not Valid`
      _))
  (set `self.PrevItemTarget` null)
  (set `self.CurrentItemTarget` null))

(fn `Get MouseLocation`
  (returns (Hit :type Boolean) (Location :type "Vector Structure"))
  (locals (HitLocation :type "Vector Structure"))
  (bind (_locationx _locationy) (`self.GetMousePosition`))
  (bind _currentitemtarget (`self.CurrentItemTarget`))
  (bind (_bblockinghit _binitialoverlap _time _distance _location) (`GameplayStatics.BreakHitResult` (`self.GetHitResultUnderCursorByChannel` "TraceTypeQuery1")))
  (bind (_worldlocation _worlddirection) (`self.DeprojectScreenPositionToWorld` _locationx _locationy))
  (if _bblockinghit
    (bind (_outhit _returnvalue) (`KismetSystemLibrary.SphereTraceSingle` (`SceneComponent.K2_GetComponentLocation` (`/Game/Blueprints/BP_Player.Camera` (`/Game/Blueprints/BP_WaveGameMode.As BP Player` (`self.As BP Wave Game Mode`)))) _location 20.0 "TraceTypeQuery2"))
    (if (not _returnvalue)
      (set `local.HitLocation` _location)
      (set `self.EnemyHit` false :!label _label)
      (`|ExecutionSequence`
        (:`then_0`
          (bind (_bblockinghit_2 _binitialoverlap_2 _time_2 _distance_2 _location_2 _impactpoint _normal _impactnormal _physmat _hitactor) (`GameplayStatics.BreakHitResult` _outhit))
          (`/Engine/EditorBlueprintResources/StandardMacros.IsValid` _hitactor
            (:`Is Valid`
              (if (`self.ActorHasTag` _hitactor "I")
                (if (not (== _hitactor (`self.CurrentItemTarget`)))
                  (`/Engine/EditorBlueprintResources/StandardMacros.IsValid` _currentitemtarget
                    (:`Is Valid`
                      (message `/Game/Blueprints/BI/BI_ItemComponant.EndHover` _currentitemtarget)
                      (set `self.PrevItemTarget` (`self.CurrentItemTarget`)))
                    (:`Is Not Valid`
                      _))
                  (set `self.CurrentItemTarget` _hitactor)
                  (message `/Game/Blueprints/BI/BI_ItemComponant.StartHover` _hitactor false null))
                (else
                  (`self.ClearItemSelect`))))))
        (:`then_1`
          (return (`self.EnemyHit`) (`local.HitLocation`)))))
    (else
      (set `local.HitLocation` (+ _worldlocation (* _worlddirection 3000)))
      (goto _label))))

(fn `Interact`
  (bind _currentitemtarget (`self.CurrentItemTarget`))
  (`/Engine/EditorBlueprintResources/StandardMacros.IsValid` _currentitemtarget
    (:`Is Valid`
      (message `/Game/Blueprints/BI/BI_ItemComponant.Interact` _currentitemtarget null))))

(fn `UserConstructionScript`)