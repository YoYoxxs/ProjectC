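; Attack component in the damage system that applies damage from hit results to actors outside the owner's team.
; DamageAllNonTeamMember loops over the hits and compares each hit actor's team number with the owner's, both read through message calls.
; Opposing actors receive the damage info through TakeDamageMessage and are recorded in a returned DamagedActor list, so repeated hits on a listed actor are skipped.
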(fn `DamageAllNonTeamMember`
  (params (Hits :type "Array of HitResult Structure") (DamageInfo :type "/Game/DamageSys/S_DamageInfo Structure"))
  (returns (ActorDamaged :type "Array of Actor Object Reference"))
  (locals (DamagedActor :type "Array of Actor Object Reference"))
  (for _array_element Hits
    (bind (_bblockinghit _binitialoverlap _time _distance _location _impactpoint _normal _impactnormal _physmat _hitactor) (`GameplayStatics.BreakHitResult` _array_element))
    (bind _teamnumber (message `/Game/DamageSys/BPI_Damagable.GetTeamNumber` _hitactor))
    (bind _teamnumber_2 (message `/Game/DamageSys/BPI_Damagable.GetTeamNumber` (`self.GetOwner`)))
    (if (and (!= _teamnumber _teamnumber_2) (not (`KismetArrayLibrary.Array_Contains` (`local.DamagedActor`) _hitactor)))
      (message `/Game/DamageSys/BPI_Damagable.TakeDamage` _hitactor DamageInfo)
      (`KismetArrayLibrary.Array_AddUnique` (`local.DamagedActor`) _hitactor)))
  (return (`local.DamagedActor`)))