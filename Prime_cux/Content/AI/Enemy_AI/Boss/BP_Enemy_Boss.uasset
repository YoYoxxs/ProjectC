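; Boss enemy Blueprint that sets up a boss health bar when play begins.
; BeginPlay runs the parent logic, calls SetWidget on its Widget with no widget supplied, then creates and stores a WBP_BossBar.
; The bar receives current and maximum health from BPCDamageSystem once, with no viewport add or later refresh in this Blueprint.
; Its MaxHealth function is a stub returning zero.
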(event `self.ReceiveBeginPlay`
  (bind _bpc_damagesystem (`self.BPC_DamageSystem`))
  (`parent.ReceiveBeginPlay`)
  (`WidgetComponent.SetWidget` (`self.Widget`) null)
  (bind _returnvalue (`|CreateWidget` "/Game/UI/Widgets/WBP_BossBar.WBP_BossBar_C"))
  (bind _output_get (set `self.BossBar` _returnvalue))
  (`/Game/UI/Widgets/WBP_BossBar.UpdateHealthPrecentage ` _output_get (`/Game/DamageSys/BPC_DamageSystem.Health` _bpc_damagesystem) (`/Game/DamageSys/BPC_DamageSystem.MaxHealth` _bpc_damagesystem)))

(fn `MaxHealth`
  (returns (MaxHealth :type "Float (double-precision)"))
  (return 0.0))

(fn `UserConstructionScript`
  (`parent.UserConstructionScript`))